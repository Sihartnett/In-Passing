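; Dialogue trigger actor that shows lines from DialogueArray on the first-person character's dialogue widget.
; On player overlap it registers as the character's CurrentDialogueBox and, unless MultiNarration is set, shows the next line with its indexed animation and a looping CenterShake.
; StartDialogue and ResetAutoplayTimer, not called here, drive AnimatedTextSwapper on a timer, advancing lines with fades until the array ends.
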(event OnComponentBeginOverlap(DialogueCollisionBox)
  (params (OverlappedComponent :type Primitive%20Component%20Object%20Reference) (OtherActor :type Actor%20Object%20Reference) (OtherComp :type Primitive%20Component%20Object%20Reference) (OtherBodyIndex :type Integer) (bFromSweep :type Boolean) (SweepResult :type Hit%20Result%20Structure%20%28by%20ref%29))
  (bind _returnvalue (Game|Player|GetPlayerPawn 0))
  (if (and (== OtherActor _returnvalue) (Variables|Default|GetisThereStillDialogue))
    (bind _asfirst_person_character (Utilities|Casting|CastToFirstPersonCharacter _returnvalue))
    (Variables|Default|Setref_FirstPersonCharacter _asfirst_person_character)
    (Variables|/Game/FirstPersonCPP/Blueprints/FirstPersonCharacter.FirstPersonCharacter_C|SetCurrent_Dialogue_Box (Variables|Default|Getref_FirstPersonCharacter) self)
    (if (not (Variables|Default|GetMultiNarration?))
      (if (== (Variables|Default|GetindexOfArray) (Variables|Default|GetSize%20of%20array))
        (Variables|Default|SetisThereStillDialogue false)
        (else
          (Variables|/Game/Widgets/Narration/W_Level1Narration.W_Level1Narration_C|SetStruct_From_Dialogue_Box (Variables|/Game/FirstPersonCPP/Blueprints/FirstPersonCharacter.FirstPersonCharacter_C|GetDialogue%20Widget%20Reference (Variables|Default|Getref_FirstPersonCharacter)) (Utilities|Array|Get(acopy) (Variables|Default|GetDialogue%20array) (Variables|Default|GetindexOfArray)))
          (Default|TextSelector (Variables|/Game/FirstPersonCPP/Blueprints/FirstPersonCharacter.FirstPersonCharacter_C|GetDialogue%20Widget%20Reference (Variables|Default|Getref_FirstPersonCharacter)))
          (Math|Integer|IncrementInt (Variables|Default|GetindexOfArray)
            (:%20%20
              (UserInterface|Animation|PlayAnimation (Variables|/Game/FirstPersonCPP/Blueprints/FirstPersonCharacter.FirstPersonCharacter_C|GetDialogue%20Widget%20Reference (Variables|Default|Getref_FirstPersonCharacter)) (Utilities|Array|Get(acopy) (Variables|/Game/Widgets/Narration/W_Level1Narration.W_Level1Narration_C|GetAnimation%20Array (Variables|/Game/FirstPersonCPP/Blueprints/FirstPersonCharacter.FirstPersonCharacter_C|GetDialogue%20Widget%20Reference (Variables|Default|Getref_FirstPersonCharacter))) (.ANimationNumber (Utilities|Struct|BreakDialogue_Struct (Variables|/Game/Widgets/Narration/W_Level1Narration.W_Level1Narration_C|GetStruct_From_Dialogue_Box (Variables|/Game/FirstPersonCPP/Blueprints/FirstPersonCharacter.FirstPersonCharacter_C|GetDialogue%20Widget%20Reference (Variables|Default|Getref_FirstPersonCharacter)))))) 0.0 1 "Forward" 1.0)
              (UserInterface|Animation|PlayAnimation (Variables|/Game/FirstPersonCPP/Blueprints/FirstPersonCharacter.FirstPersonCharacter_C|GetDialogue%20Widget%20Reference (Variables|Default|Getref_FirstPersonCharacter)) (Variables|/Game/Widgets/Narration/W_Level1Narration.W_Level1Narration_C|GetCenterShake (Variables|/Game/FirstPersonCPP/Blueprints/FirstPersonCharacter.FirstPersonCharacter_C|GetDialogue%20Widget%20Reference (Variables|Default|Getref_FirstPersonCharacter))) 0.0 0 "Forward" 1.0))))))))

(event Custom|Reset%20Autoplay%20Timer
  ;[1 1 1] Begin Animation on Overlap, Rest auto timer, start dialogue, and change text.
  (Utilities|Time|ClearandInvalidateTimerbyHandle (Variables|Default|Getref_AutoScroll_Timer))
  (bind _returnvalue (Utilities|Time|SetTimerbyEvent (delegate Custom|AnimatedTextSwapper) 5.0 (Variables|Default|GetisThereStillDialogue)))
  (Variables|Default|Setref_AutoScroll_Timer _returnvalue))

(event Custom|Start%20Dialogue
  ;[1 1 1] Begin Animation on Overlap, Rest auto timer, start dialogue, and change text.
  (CallFunction|AnimatedTextSwapper)
  (bind _returnvalue (Utilities|Time|SetTimerbyEvent (delegate Custom|AnimatedTextSwapper) 5.0 (Variables|Default|GetisThereStillDialogue)))
  (Variables|Default|Setref_AutoScroll_Timer _returnvalue))

(event Custom|AnimatedTextSwapper
  (bind _ref_firstpersoncharacter (Variables|Default|Getref_FirstPersonCharacter))
  (bind _ref_firstpersoncharacter_2 (Variables|Default|Getref_FirstPersonCharacter))
  (bind _ref_firstpersoncharacter_3 (Variables|Default|Getref_FirstPersonCharacter))
  (bind _dialogue_widget_reference (Variables|/Game/FirstPersonCPP/Blueprints/FirstPersonCharacter.FirstPersonCharacter_C|GetDialogue%20Widget%20Reference _ref_firstpersoncharacter))
  (bind _dialogue_widget_reference_2 (Variables|/Game/FirstPersonCPP/Blueprints/FirstPersonCharacter.FirstPersonCharacter_C|GetDialogue%20Widget%20Reference _ref_firstpersoncharacter_2))
  (bind _dialogue_widget_reference_3 (Variables|/Game/FirstPersonCPP/Blueprints/FirstPersonCharacter.FirstPersonCharacter_C|GetDialogue%20Widget%20Reference _ref_firstpersoncharacter_3))
  ;[1 1 1] Begin Animation on Overlap, Rest auto timer, start dialogue, and change text.
  (if (== (Variables|Default|GetindexOfArray) 0)
    _
    (else
      (Class|UserWidget|StopAnimation _dialogue_widget_reference (Utilities|Array|Get(acopy) (Variables|/Game/Widgets/Narration/W_Level1Narration.W_Level1Narration_C|GetAnimation%20Array _dialogue_widget_reference) (.ANimationNumber (Utilities|Struct|BreakDialogue_Struct (Variables|/Game/Widgets/Narration/W_Level1Narration.W_Level1Narration_C|GetStruct_From_Dialogue_Box _dialogue_widget_reference)))))
      (CallFunction|FadeOutTextSwagger)))
  (if (== (Variables|Default|GetindexOfArray) (Variables|Default|GetSize%20of%20array))
    (Variables|Default|SetisThereStillDialogue false)
    (CallFunction|FadeOutTextSwagger)
    (Utilities|Time|ClearandInvalidateTimerbyHandle (Variables|Default|Getref_AutoScroll_Timer))
    (else
      (Variables|/Game/Widgets/Narration/W_Level1Narration.W_Level1Narration_C|SetStruct_From_Dialogue_Box _dialogue_widget_reference_3 (Utilities|Array|Get(acopy) (Variables|Default|GetDialogue%20array) (Variables|Default|GetindexOfArray)))
      (Default|TextSelector _dialogue_widget_reference_3)
      (Math|Integer|IncrementInt (Variables|Default|GetindexOfArray)
        (:%20%20
          (CallFunction|FadeinTextSwapper)
          (UserInterface|Animation|PlayAnimation _dialogue_widget_reference_2 (Utilities|Array|Get(acopy) (Variables|/Game/Widgets/Narration/W_Level1Narration.W_Level1Narration_C|GetAnimation%20Array _dialogue_widget_reference_2) (.ANimationNumber (Utilities|Struct|BreakDialogue_Struct (Variables|/Game/Widgets/Narration/W_Level1Narration.W_Level1Narration_C|GetStruct_From_Dialogue_Box _dialogue_widget_reference_2)))) 0.0 0 "Forward" 1.0))))))

(event Custom|FadeInTextSwapper
  (bind _ref_firstpersoncharacter (Variables|Default|Getref_FirstPersonCharacter))
  (bind _dialogue_widget_reference (Variables|/Game/FirstPersonCPP/Blueprints/FirstPersonCharacter.FirstPersonCharacter_C|GetDialogue%20Widget%20Reference _ref_firstpersoncharacter))
  (UserInterface|Animation|PlayAnimation _dialogue_widget_reference (Variables|/Game/Widgets/Narration/W_Level1Narration.W_Level1Narration_C|GetFadeIn _dialogue_widget_reference) 0.0 1 "Forward" 1.0))

(event Custom|FadeInStop
  (bind _ref_firstpersoncharacter (Variables|Default|Getref_FirstPersonCharacter))
  (bind _dialogue_widget_reference (Variables|/Game/FirstPersonCPP/Blueprints/FirstPersonCharacter.FirstPersonCharacter_C|GetDialogue%20Widget%20Reference _ref_firstpersoncharacter))
  (Class|UserWidget|StopAnimation _dialogue_widget_reference (Variables|/Game/Widgets/Narration/W_Level1Narration.W_Level1Narration_C|GetFadeIn _dialogue_widget_reference)))

(event Custom|FadeOutTextSwagger
  (bind _ref_firstpersoncharacter (Variables|Default|Getref_FirstPersonCharacter))
  (bind _dialogue_widget_reference (Variables|/Game/FirstPersonCPP/Blueprints/FirstPersonCharacter.FirstPersonCharacter_C|GetDialogue%20Widget%20Reference _ref_firstpersoncharacter))
  (UserInterface|Animation|PlayAnimation _dialogue_widget_reference (Variables|/Game/Widgets/Narration/W_Level1Narration.W_Level1Narration_C|GetFadeOut _dialogue_widget_reference) 0.0 1 "Forward" 1.0))

(event Custom|FadeOutStop
  (bind _ref_firstpersoncharacter (Variables|Default|Getref_FirstPersonCharacter))
  (bind _dialogue_widget_reference (Variables|/Game/FirstPersonCPP/Blueprints/FirstPersonCharacter.FirstPersonCharacter_C|GetDialogue%20Widget%20Reference _ref_firstpersoncharacter))
  (Class|UserWidget|StopAnimation _dialogue_widget_reference (Variables|/Game/Widgets/Narration/W_Level1Narration.W_Level1Narration_C|GetFadeOut _dialogue_widget_reference)))

(event EventBeginPlay
  (Variables|Default|SetSize%20of%20array (Utilities|Array|Length (Variables|Default|GetDialogue%20array))))

(fn ConstructionScript)