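; BP_LampTree is a lamp tree prop whose lamp swings while the player is inside its trigger volume.
; Overlap begin and end on StartSwingingVolume, filtered to player pawn 0, start and stop the LampSwing timeline.
; The timeline drives the lamp's world roll with pitch and yaw held at zero, restarting from the beginning on entry and halting in place on exit.
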(event OnComponentBeginOverlap(StartSwingingVolume)
  (params (OverlappedComponent :type Primitive%20Component%20Object%20Reference) (OtherActor :type Actor%20Object%20Reference) (OtherComp :type Primitive%20Component%20Object%20Reference) (OtherBodyIndex :type Integer) (bFromSweep :type Boolean) (SweepResult :type Hit%20Result%20Structure%20%28by%20ref%29))
  (if (== OtherActor (Game|Player|GetPlayerPawn 0))
    (CallFunction|BeginSwing)))

(event OnComponentEndOverlap(StartSwingingVolume)
  (params (OverlappedComponent :type Primitive%20Component%20Object%20Reference) (OtherActor :type Actor%20Object%20Reference) (OtherComp :type Primitive%20Component%20Object%20Reference) (OtherBodyIndex :type Integer))
  (if (== OtherActor (Game|Player|GetPlayerPawn 0))
    (CallFunction|StopSwing)))

(event Custom|BeginSwing
  (bind _newtrack_0 (Timeline|LampSwing PlayFromStart)
    (:Update
      (Transformation|SetWorldRotation (Variables|Default|GetLamp) (Math|Rotator|MakeRotator _newtrack_0 0.0 0.0) false false))))

(event Custom|StopSwing
  (bind _newtrack_0 (Timeline|LampSwing Stop)
    (:Update
      (Transformation|SetWorldRotation (Variables|Default|GetLamp) (Math|Rotator|MakeRotator _newtrack_0 0.0 0.0) false false))))

(fn ConstructionScript)