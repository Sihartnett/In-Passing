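; Game mode for a first-person platformer, handling screen effects, player death and respawn.
; BeginPlay caches overlay widgets, the first post-process volume and the character; helper functions show several overlays and brighten lights.
; PlayerDeath teleports the player to SpawnLocation, resets breaking platforms and destroys projectiles.
; AdjustPlayerHealth is meant to drive saturation and vignette from health, but its health inputs are unwired, so its zero-to-zero comparison always triggers death.
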(event Custom|WaitToShake
  (Utilities|FlowControl|Delay 1.0)
  (Variables|/Script/Unbelievable.UnbelievableCharacter|SetshouldShake (.AsFirst%20Person%20Character (Utilities|Casting|CastToFirstPersonCharacter (Game|Player|GetPlayerPawn 0))) true))

(event EventBeginPlay
  (Variables|Default|SetREFPlayerController (Game|GetPlayerController 0))
  (bind _returnvalue (UserInterface|CreateWidget "/Game/Widgets/W_DeathFade.W_DeathFade_C" (Variables|Default|GetREFPlayerController)))
  (Variables|Default|SetDeathFade _returnvalue)
  (bind _returnvalue_2 (UserInterface|CreateWidget "/Game/Widgets/Thanks_for_Playing.Thanks_for_Playing_C" (Variables|Default|GetREFPlayerController)))
  (Variables|Default|SetThanksForPlaying _returnvalue_2)
  (bind _returnvalue_3 (UserInterface|CreateWidget "/Game/Widgets/W_TransitionFadeOut.W_TransitionFadeOut_C" (Variables|Default|GetREFPlayerController)))
  (Variables|Default|SetTransitionFade _returnvalue_3)
  (bind _returnvalue_4 (UserInterface|CreateWidget "/Game/Widgets/W_ChargedPlatformFlash.W_ChargedPlatformFlash_C" (Variables|Default|GetREFPlayerController)))
  (Variables|Default|SetChargedPlatformFlash _returnvalue_4)
  (bind _returnvalue_5 (UserInterface|CreateWidget "/Game/Widgets/W_IceRim1.W_IceRim1_C" (Variables|Default|GetREFPlayerController)))
  (Variables|Default|SetIceRimLerp _returnvalue_5)
  (bind _returnvalue_6 (UserInterface|CreateWidget "/Game/Widgets/W_OrbPickupRim.W_OrbPickupRim_C" (Variables|Default|GetREFPlayerController)))
  (Variables|Default|SetOrbPickupRim _returnvalue_6)
  (bind _outactors (Actor|GetAllActorsOfClass "/Script/Engine.PostProcessVolume"))
  (bind _output_get (Variables|Default|Setprocess%20volume (Utilities|Array|Get(acopy) _outactors)))
  (bind _structout (Utilities|Struct|SetmembersinPostProcessSettings (Variables|/Script/Engine.PostProcessVolume|GetSettings _output_get) (Math|Vector4|MakeVector4 1.0 1.0 1.0 1.0) 0.0 0.0))
  (Variables|/Script/Engine.PostProcessVolume|SetSettings _output_get _structout)
  (bind _asfirst_person_character (Utilities|Casting|CastToFirstPersonCharacter (Game|GetPlayerCharacter 0))
    (:then
      (bind _output_get_2 (Variables|Default|Setcharacter%20reference _asfirst_person_character))
      (Development|PrintString (Utilities|String|Append "Ths is the name of the player: " (Utilities|GetDisplayName _output_get_2))))
    (:CastFailed
      (Development|PrintString "We have no Unbelieveable character in Game Mode"))))

(event EventTick
  (params (DeltaSeconds :type Float%20%28single-precision%29)))

(fn ConstructionScript)

(fn PlayerDeath
  (bind _returnvalue (Game|Player|GetPlayerPawn 0))
  (bind _spawnlocation (Variables|Default|GetSpawnLocation))
  (bind _asfirst_person_character (Utilities|Casting|CastToFirstPersonCharacter _returnvalue))
  (Variables|/Script/Unbelievable.UnbelievableCharacter|SetshouldShake _asfirst_person_character false)
  (Variables|/Script/Engine.MovementComponent|SetVelocity (Variables|/Script/Engine.Character|GetCharacterMovement _asfirst_person_character) "0, 0, 0")
  (Transformation|SetActorLocation _asfirst_person_character (.location _spawnlocation) false false)
  (Pawn|SetControlRotation (Game|GetPlayerController 0) (.rotation _spawnlocation))
  (Default|CallDeathEvents)
  ;[1 1 1] Reset Breaking Platforms
  (bind _outactors (Actor|GetAllActorswithTag "BreakingPlatform"))
  (for _array_element _outactors
    (bind _asbp_breaking_platform_2 (Utilities|Casting|CastToBP_BreakingPlatform2 _array_element)
      (:then
        (Default|ResetPos _asbp_breaking_platform_2))
      (:CastFailed
        _))
    (bind _asbp_breaking_platform_2_2 (Utilities|Casting|CastToBP_BreakingPlatform2 _array_element))
    (Default|ResetPos _asbp_breaking_platform_2_2)
    (CallFunction|WaittoShake))
  (bind _outactors_2 (Actor|GetAllActorsOfClass "/Game/Blueprints/BP_Projectile.BP_Projectile_C"))
  (for _array_element_2 _outactors_2
    (Actor|DestroyActor _array_element_2)))

(fn Fadein
  (UserInterface|Viewport|AddtoViewport (Variables|Default|GetDeathFade) 0))

(fn LightIncrease
  (params (LightComponent :type Light%20Component%20Object%20Reference) (LevelLight :type Light%20Component%20Base%20Object%20Reference))
  (Rendering|Components|Light|SetIntensity LightComponent (+ (Variables|/Script/Engine.LightComponentBase|GetIntensity LevelLight) (Variables|Default|GetLightIncreaseAmount))))

(fn ChargedPlatformFade
  (UserInterface|Viewport|AddtoViewport (Variables|Default|GetChargedPlatformFlash) 0))

(fn IcePlatformRim
  (bind _icerimlerp (Variables|Default|GetIceRimLerp))
  (if (not (UserInterface|Viewport|IsinViewport _icerimlerp))
    (UserInterface|Viewport|AddtoViewport _icerimlerp 0)))

(fn OrbCollectionRim
  (UserInterface|Viewport|AddtoViewport (Variables|Default|GetOrbPickupRim) 0))

(fn AdjustPlayerHealth
  (bind _returnvalue (Math|Conversions|ToFloat(Integer) 0))
  (bind _returnvalue_2 (Math|Conversions|ToFloat(Integer) 0))
  (bind _process_volume (Variables|Default|Getprocess%20volume))
  (bind _process_volume_2 (Variables|Default|Getprocess%20volume))
  (bind _returnvalue_3 (/ _returnvalue_2 _returnvalue))
  (bind _returnvalue_4 (- _returnvalue_3 1.0))
  (bind _returnvalue_5 (Math|Float|Absolute(Float) _returnvalue_4))
  (bind _structout (Utilities|Struct|SetmembersinPostProcessSettings (Variables|/Script/Engine.PostProcessVolume|GetSettings _process_volume) (Math|Vector4|MakeVector4 1.0 1.0 1.0 _returnvalue_3) (* _returnvalue_5 5.0) _returnvalue_5))
  (Variables|/Script/Engine.PostProcessVolume|SetSettings _process_volume _structout)
  (Math|Float|CompareFloat 0.0 0.0
    (:==
      _)
    (:<
      _))
  (CallFunction|Fadein)
  (CallFunction|PlayerDeath)
  (Variables|/Script/Unbelievable.UnbelievableCharacter|SethealthPoints (Variables|Default|Getcharacter%20reference) 0.0)
  (bind _structout_2 (Utilities|Struct|SetmembersinPostProcessSettings (Variables|/Script/Engine.PostProcessVolume|GetSettings _process_volume_2) (Math|Vector4|MakeVector4 1.0 1.0 1.0 1.0) 0.0 0.0))
  (Variables|/Script/Engine.PostProcessVolume|SetSettings _process_volume_2 _structout_2))