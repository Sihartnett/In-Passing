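; BP_PlayerRespawn is a checkpoint actor that updates the player's spawn point and saves progress on overlap.
; BeginPlay caches the game mode, game instance and file-system data handler.
; Each player overlap takes a screenshot and passes death count, mode and level from the game instance to the character.
; A DoOnce then registers this checkpoint with the game mode, saves the game with its transform and resets the death count.
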(event EventBeginPlay
  ;[1 1 1] Set Refs
  (bind _asbp_game_mode (Utilities|Casting|CastToBP_GameMode (Game|GetGameMode)))
  (Variables|Default|SetREFGameMode _asbp_game_mode)
  (bind _asbp_game_instance (Utilities|Casting|CastToBP_GameInstance (Game|GetGameInstance)))
  (Variables|Default|Setref_BPGameInstance _asbp_game_instance)
  (bind _outactors (Actor|GetAllActorsOfClass "/Game/Blueprints/BP_Data_handler_For_File_System.BP_Data_handler_For_File_System_C"))
  (Variables|Default|SetData_Holder_Variable (Utilities|Array|Get(acopy) _outactors)))

(event Collision|EventActorBeginOverlap
  (params (OtherActor :type Actor%20Object%20Reference))
  (bind _refgamemode (Variables|Default|GetREFGameMode))
  (bind _ref_bpgameinstance (Variables|Default|Getref_BPGameInstance))
  ;[1 1 1] Setting This Spawn Loc on Overlap
  (if (== OtherActor (Game|Player|GetPlayerPawn 0))
    (Utilities|FlowControl|Sequence
      (:then_0
        (bind _asfirst_person_character (Utilities|Casting|CastToFirstPersonCharacter (Game|GetPlayerCharacter 0)))
        (bind _output_get (Variables|Default|Setour_UnbelievableCharacter _asfirst_person_character))
        (Default|Screenshot _asfirst_person_character)
        (Class|UnbelievableCharacter|SetAllVariablesNecessaryfromBlueprint _output_get (Variables|/Game/Blueprints/BP_GameInstance.BP_GameInstance_C|GetNumberOfDeaths _ref_bpgameinstance) (Variables|/Game/Blueprints/BP_GameInstance.BP_GameInstance_C|GetgameModeSelected _ref_bpgameinstance) (Variables|/Game/Blueprints/BP_GameInstance.BP_GameInstance_C|GetLevel_Selected _ref_bpgameinstance)))
      (:then_1
        (Utilities|FlowControl|DoOnce false
          (:Completed
            (bind _output_get_2 (Variables|/Game/Blueprints/BP_GameMode.BP_GameMode_C|SetSpawnLocation _refgamemode (Transformation|GetActorTransform)))
            (Variables|/Game/Blueprints/BP_GameMode.BP_GameMode_C|SetActiveSpawnPoint _refgamemode self)
            (Variables|/Script/Unbelievable.UnbelievableCharacter|SetlocationToSet (Variables|Default|Getour_UnbelievableCharacter) (.location _output_get_2))
            (Variables|/Script/Unbelievable.UnbelievableCharacter|SetrotationToSet (Variables|Default|Getour_UnbelievableCharacter) (Transformation|GetActorRotation))
            (Class|UnbelievableCharacter|SaveGame (Variables|Default|Getour_UnbelievableCharacter))
            (Default|ResetDeathCount _asfirst_person_character)))))))

(fn ConstructionScript)