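; BP_Locket_Vignette9 is a locket actor that rotates every tick and can hover and fade out.
; Once Hover is called, two timelines alternately lerp it between its start location and an offset; separate events stop each timeline.
; Fadeout animates a scalar on a new dynamic material instance, never assigned to the pendant, then swaps in a fixed material.
; BeginPlay only caches locations; the delayed Hover start is disconnected.
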(event Custom|Hover
  (bind _floatlerp (Timeline|Timeline_0 PlayFromStart)
    (:Update
      (Transformation|SetActorLocation (Math|Vector|Lerp(Vector) (Variables|Default|GetREFOriginalLoc) (Variables|Default|GetREFHoverDestination) _floatlerp) false false))
    (:Finished
      (CallFunction|HoverReverse))))

(event Custom|HoverReverse
  (bind _floatlerp (Timeline|Timeline_1 PlayFromStart)
    (:Update
      (Transformation|SetActorLocation (Math|Vector|Lerp(Vector) (Variables|Default|GetREFHoverDestination) (Variables|Default|GetREFOriginalLoc) _floatlerp) false false))
    (:Finished
      (CallFunction|Hover))))

(event Custom|timeline%20stop%202
  (bind _floatlerp (Timeline|Timeline_0 Stop)
    (:Update
      (Transformation|SetActorLocation (Math|Vector|Lerp(Vector) (Variables|Default|GetREFOriginalLoc) (Variables|Default|GetREFHoverDestination) _floatlerp) false false))
    (:Finished
      (CallFunction|HoverReverse))))

(event Custom|timeline%20stop
  (bind _floatlerp (Timeline|Timeline_1 Stop)
    (:Update
      (Transformation|SetActorLocation (Math|Vector|Lerp(Vector) (Variables|Default|GetREFHoverDestination) (Variables|Default|GetREFOriginalLoc) _floatlerp) false false))
    (:Finished
      (CallFunction|Hover))))

(event Custom|Fade%20out
  (bind _returnvalue (Rendering|Material|CreateDynamicMaterialInstance (Rendering|Material|GetMaterial (Variables|Default|GetLocketPendant) 0) "None" :!class /Script/Engine.KismetMaterialLibrary))
  (bind _newtrack_0 (Timeline|LightFade PlayFromStart)
    (:Update
      (Rendering|Material|SetScalarParameterValue _returnvalue "Param" _newtrack_0 :!class /Script/Engine.MaterialInstanceDynamic))
    (:Finished
      (Rendering|Material|SetMaterial (Variables|Default|GetLocketPendant) 0 "/Game/Assets/Vignettes/Vignette_6/Mesh_Textures/Materials/Locket_Pendant_txtr.Locket_Pendant_txtr"))))

(event EventBeginPlay
  (bind _output_get (Variables|Default|SetREFOriginalLoc (Transformation|GetActorLocation)))
  (Variables|Default|SetREFHoverDestination (- _output_get (Variables|Default|GetMovement%20Amount))))

(event EventTick
  (params (DeltaSeconds :type Float%20%28single-precision%29))
  (Transformation|AddActorLocalRotation (Variables|Default|GetRotation%20Rate) false false))

(fn ConstructionScript)