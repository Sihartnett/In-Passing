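; BP_Projectile is a homing projectile that chases the player with an attached approach sound and destroys itself after its lifespan.
; On overlapping the player, the selected game mode in BP_GameInstance decides between health loss with healing interrupted, harmless removal, or instant death with a fade widget.
; A second volume flags when the player is within dodge range for the tutorial.
; Disconnected nodes hold unused directional-volume and debug experiments.
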(event OnComponentEndOverlap(Tut_DodgeCheckVolume)
  (params (OverlappedComponent :type Primitive%20Component%20Object%20Reference) (OtherActor :type Actor%20Object%20Reference) (OtherComp :type Primitive%20Component%20Object%20Reference) (OtherBodyIndex :type Integer))
  (bind _refplayercharacter (Variables|Default|GetREFPlayerCharacter))
  (if (== OtherActor _refplayercharacter)
    (Variables|/Game/FirstPersonCPP/Blueprints/FirstPersonCharacter.FirstPersonCharacter_C|SetTut_isInDodgeVolume _refplayercharacter false)))

(event OnComponentBeginOverlap(Tut_DodgeCheckVolume)
  (params (OverlappedComponent :type Primitive%20Component%20Object%20Reference) (OtherActor :type Actor%20Object%20Reference) (OtherComp :type Primitive%20Component%20Object%20Reference) (OtherBodyIndex :type Integer) (bFromSweep :type Boolean) (SweepResult :type Hit%20Result%20Structure%20%28by%20ref%29))
  (bind _refplayercharacter (Variables|Default|GetREFPlayerCharacter))
  (if (== OtherActor _refplayercharacter)
    (Variables|/Game/FirstPersonCPP/Blueprints/FirstPersonCharacter.FirstPersonCharacter_C|SetTut_isInDodgeVolume _refplayercharacter true)))

(event OnComponentBeginOverlap(Collision)
  (params (OverlappedComponent :type Primitive%20Component%20Object%20Reference) (OtherActor :type Actor%20Object%20Reference) (OtherComp :type Primitive%20Component%20Object%20Reference) (OtherBodyIndex :type Integer) (bFromSweep :type Boolean) (SweepResult :type Hit%20Result%20Structure%20%28by%20ref%29))
  (bind _refplayercharacter (Variables|Default|GetREFPlayerCharacter))
  (bind _refplayercharacter_2 (Variables|Default|GetREFPlayerCharacter))
  ;[1 1 1] Temp Projectile Functionality
  (if (== OtherActor (Game|Player|GetPlayerPawn 0))
    (switch int (Variables|/Game/Blueprints/BP_GameInstance.BP_GameInstance_C|GetgameModeSelected (Variables|Default|Getref_GameInstance))
      (:0
        (Variables|/Script/Unbelievable.UnbelievableCharacter|SethealthPoints _refplayercharacter (- (Variables|/Script/Unbelievable.UnbelievableCharacter|GethealthPoints _refplayercharacter) 1.0) :!label _label)
        (Audio|PlaySound2D (Utilities|Array|Get(acopy) (Variables|Default|GetHitSoundsArray) (Math|Random|RandomIntegerinRange 0 3)) 0.5 0.9 0.0 0 0)
        (Variables|/Script/Unbelievable.UnbelievableCharacter|SetdamageHasBeenTaken _refplayercharacter true)
        (Variables|/Script/Unbelievable.UnbelievableCharacter|SethealthTimer _refplayercharacter 0.0)
        (Variables|/Script/Unbelievable.UnbelievableCharacter|SetshouldBeHealing _refplayercharacter_2 false)
        (Default|StopHeal _refplayercharacter_2)
        (Default|AlterVisualforHealth _refplayercharacter_2)
        (Actor|DestroyActor :!label _label_2))
      (:1
        (goto _label_2))
      (:2
        (goto _label))
      (:3
        (goto _label))
      (:4
        (Audio|PlaySound2D "/Game/Audio_Files/death_from_projectile.death_from_projectile" 1.0 1.0 0.0 0 0)
        (bind _returnvalue (UserInterface|CreateWidget "/Game/Widgets/W_DeathFade.W_DeathFade_C" (Game|GetPlayerController 0)))
        (UserInterface|Viewport|AddtoViewport _returnvalue 0)
        (Default|PlayerDeath (.AsBP%20Game%20Mode (Utilities|Casting|CastToBP_GameMode (Game|GetGameMode))))
        (Actor|DestroyActor)))))

(event EventBeginPlay
  (bind _returnvalue (Game|Player|GetPlayerPawn 0))
  (bind _sphere (Variables|Default|GetSphere))
  (bind _asfirst_person_character (Utilities|Casting|CastToFirstPersonCharacter _returnvalue))
  (Audio|SpawnSoundAttached "/Game/Audio_Files/projectile_approaching.projectile_approaching" _sphere "None" (Transformation|GetWorldLocation _sphere) "0, 0, 0" "KeepWorldPosition" true 0.33 0.9 0.0 "/Game/Audio_Files/Sound_Cues/NewSoundAttenuation.NewSoundAttenuation" 0)
  ;[1 1 1] Set Refs and Proj Lifespan
  (bind _asbp_game_instance (Utilities|Casting|CastToBP_GameInstance (Game|GetGameInstance)))
  (Variables|Default|Setref_GameInstance _asbp_game_instance)
  (Variables|/Script/Engine.ProjectileMovementComponent|SetHomingTargetComponent (Variables|Default|GetProjectileMovement) (Variables|/Script/Engine.Character|GetCapsuleComponent _asfirst_person_character))
  (Variables|Default|SetREFPlayerCharacter _asfirst_person_character)
  (Utilities|FlowControl|Delay (Variables|Default|GetProjectileLifespan))
  (Actor|DestroyActor))

(event EventTick
  (params (DeltaSeconds :type Float%20%28single-precision%29)))

(fn ConstructionScript)

(fn PlayerRefPass
  (return false))