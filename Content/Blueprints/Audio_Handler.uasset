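; Audio handler actor that plays a sound when the player enters its SoundLimit area, stops it when the player leaves, and resumes from the tracked position on re-entry.
; Only the first player overlap starts from zero; any other begin overlap plays from CurrentPlayTime and resets a DoOnce.
; Playback-percent updates feed that DoOnce, which saves the resume offset, wrapped past the sound's duration, and opens a Gate that updates CurrentPlayTime.
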(event OnComponentBeginOverlap(SoundLimit)
  (params (OverlappedComponent :type Primitive%20Component%20Object%20Reference) (OtherActor :type Actor%20Object%20Reference) (OtherComp :type Primitive%20Component%20Object%20Reference) (OtherBodyIndex :type Integer) (bFromSweep :type Boolean) (SweepResult :type Hit%20Result%20Structure%20%28by%20ref%29))
  (bind _sound_effect_component (Variables|Default|GetSound%20Effect%20component))
  (if (and (== (Game|Player|GetPlayerPawn 0) OtherActor) (Variables|Default|GetFirstTime))
    (Audio|Components|Audio|Play _sound_effect_component 0.0)
    (Variables|Default|SetFirstTime false)
    (else
      (Audio|Components|Audio|Play _sound_effect_component (Variables|Default|GetCurrentPlayTime))
      (Utilities|FlowControl|DoOnce false) ; enters at Reset
    )))

(event OnComponentEndOverlap(SoundLimit)
  (params (OverlappedComponent :type Primitive%20Component%20Object%20Reference) (OtherActor :type Actor%20Object%20Reference) (OtherComp :type Primitive%20Component%20Object%20Reference) (OtherBodyIndex :type Integer))
  (if (== (Game|Player|GetPlayerPawn 0) OtherActor)
    (Audio|Components|Audio|Stop (Variables|Default|GetSound%20Effect%20component))
    (Utilities|FlowControl|Gate true) ; enters at Close
  ))

(event OnAudioPlaybackPercent(SoundEffectcomponent)
  (params (PlayingSoundWave :type Sound%20Wave%20Object%20Reference) (PlaybackPercent :type Float%20%28single-precision%29))
  (Utilities|FlowControl|Sequence
    (:then_0
      (Utilities|FlowControl|DoOnce false
        (:Completed
          (if (>= (Variables|Default|GetCurrentPlayTime) (Variables|/Script/Engine.SoundBase|GetDuration PlayingSoundWave))
            (Variables|Default|SetPreviousPlayTime (- (Variables|Default|GetCurrentPlayTime) (Variables|/Script/Engine.SoundBase|GetDuration PlayingSoundWave)))
            (goto _label Open)
            (else
              (Variables|Default|SetPreviousPlayTime (Variables|Default|GetCurrentPlayTime))
              (goto _label Open))))))
    (:then_1
      (Utilities|FlowControl|Gate true :!label _label
        (:Exit
          (Variables|Default|SetCurrentPlayTime (+ (/ (* (Variables|/Script/Engine.SoundBase|GetDuration PlayingSoundWave) (* PlaybackPercent 1e+02)) 1e+02) (Variables|Default|GetPreviousPlayTime))))))))

(event EventBeginPlay)

(event Collision|EventActorBeginOverlap
  (params (OtherActor :type Actor%20Object%20Reference)))

(event EventTick
  (params (DeltaSeconds :type Float%20%28single-precision%29)))

(fn ConstructionScript)