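; A light orb pickup that, once activated, opens the way to the next level.
; LightActivate makes the orb emissive, raises it from its start position on a timeline, then plays a sound and spawns BP_LoadNextLevel at a hard-coded transform.
; The player's first overlap calls LightPickUp on FirstPersonCharacter and destroys the orb when the LerpFade timeline finishes.
; Hover, material fade and game-mode collection logic are left disconnected.
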(event OnComponentBeginOverlap(PickupVolume)
  (params (OverlappedComponent :type Primitive%20Component%20Object%20Reference) (OtherActor :type Actor%20Object%20Reference) (OtherComp :type Primitive%20Component%20Object%20Reference) (OtherBodyIndex :type Integer) (bFromSweep :type Boolean) (SweepResult :type Hit%20Result%20Structure%20%28by%20ref%29))
  (if (== OtherActor (Game|Player|GetPlayerPawn 0))
    (Utilities|FlowControl|DoOnce false
      (:Completed
        (bind _asfirst_person_character (Utilities|Casting|CastToFirstPersonCharacter OtherActor))
        (Default|LightPickUp _asfirst_person_character)
        (bind _newtrack_0 (Timeline|LerpFade PlayFromStart)
          (:Finished
            (Actor|DestroyActor)))))))

(event Custom|HoverStart)

(event Custom|LightActivate
  (bind _startloc (Variables|Default|GetStartLoc))
  (bind _returnvalue (+ _startloc "0, 0,130.000000"))
  (Rendering|Material|SetMaterial (Variables|Default|GetOrb) 0 "/Game/Particles/M_EmissiveLight.M_EmissiveLight")
  (bind _newtrack_0 (Timeline|Timeline_0 PlayFromStart)
    (:Update
      (Transformation|SetActorLocation (Math|Vector|Lerp(Vector) _startloc _returnvalue _newtrack_0) false false))
    (:Finished
      (Audio|SpawnSoundatLocation "/Game/Audio_Files/LightActivationSound.LightActivationSound" _returnvalue "0, 0, 0" 1.0 1.0 0.0 "/Game/Audio_Files/LightActivationAttenuation.LightActivationAttenuation" 0)
      (Game|SpawnActorfromClass "/Game/Blueprints/BP_LoadNextLevel.BP_LoadNextLevel_C" (Math|Transform|MakeTransform "-9587.000000,-10704.728516,16373.330078" "0, 0, 0" "5.000000,4.250000,6.437500") "Undefined" 0 0))))

(event EventBeginPlay
  (Variables|Default|SetStartLoc (Transformation|GetActorLocation)))

(fn ConstructionScript)