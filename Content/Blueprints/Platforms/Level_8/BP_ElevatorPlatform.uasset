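; BP_ElevatorPlatform is a Level 8 moving platform that travels in one direction on an endless loop after a configurable start delay.
; BeginPlay caches the start transform and turns AmountToMove into the end transform by subtracting its location from the start location, keeping rotation and scale.
; FallingTimeline lerps the platform to that end without sweeping, then snaps it back to the start and replays after a brief pause.
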(event Custom|StartFall
  (bind _newtrack_0 (Timeline|Falling%20Timeline PlayFromStart)
    (:Update
      (Transformation|SetActorTransform (Math|Transform|Lerp(Transform) (Variables|Default|GetStartLoc) (Variables|Default|GetAmountToMove) _newtrack_0)))
    (:Finished
      (Transformation|SetActorTransform (Variables|Default|GetStartLoc))
      (Utilities|FlowControl|Delay 0.1)
      (CallFunction|StartFall))))

(event EventBeginPlay
  (Variables|Default|SetStartLoc (Transformation|GetActorTransform))
  (Variables|Default|SetAmountToMove (Math|Transform|MakeTransform (- (.location (Variables|Default|GetStartLoc)) (.location (Variables|Default|GetAmountToMove))) (.rotation (Variables|Default|GetStartLoc)) (.scale (Variables|Default|GetStartLoc))))
  (Utilities|FlowControl|Delay (Variables|Default|GetStart%20Delay))
  (CallFunction|StartFall))

(event Collision|EventActorBeginOverlap
  (params (OtherActor :type Actor%20Object%20Reference)))

(event EventTick
  (params (DeltaSeconds :type Float%20%28single-precision%29)))

(fn ConstructionScript)