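; Level 7 breakable platform that rumbles and falls when the player pawn hits it.
; The hit plays the Break timeline, which moves the actor by lerping from its current location toward a track-driven offset each update.
; From BeginPlay, a self-restarting timeline continuously rotates the Platform component as an idle shake.
; ResetPos, meant for player death, restores the transform saved at BeginPlay and stops the break.
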(event Custom|StaticShake
  (bind _newtrack_0 (Timeline|Timeline_0 PlayFromStart)
    (:Update
      (Transformation|SetWorldRotation (Variables|Default|GetPlatform) (Math|Rotator|MakeRotator (.x _newtrack_0) (.y _newtrack_0) (.z _newtrack_0)) false false))
    (:Finished
      (CallFunction|StaticShake))))

(event Custom|ResetPos
  (bind _returnvalue (Transformation|GetActorLocation))
  (bind _reftransform (Variables|Default|GetREFTransform))
  ;[1 1 1] Reset On Player Death
  (Transformation|SetActorLocationAndRotation (.location _reftransform) (.rotation _reftransform))
  ;[1 1 1] Rumble and Fall
  (bind (_direction _newtrack_0 _newtrack_1) (Timeline|Break Stop)
    (:Update
      (Transformation|SetActorLocation (Math|Vector|Lerp(Vector) _returnvalue (+ _returnvalue _newtrack_1) _newtrack_0) false false))))

(event EventBeginPlay
  ;[1 1 1] Set Loc Ref
  (Variables|Default|SetREFTransform (Transformation|GetActorTransform))
  (CallFunction|StaticShake))

(event Collision|EventHit
  (params (MyComp :type Primitive%20Component%20Object%20Reference) (Other :type Actor%20Object%20Reference) (OtherComp :type Primitive%20Component%20Object%20Reference) (bSelfMoved :type Boolean) (HitLocation :type Vector :default "0, 0, 0") (HitNormal :type Vector :default "0, 0, 0") (NormalImpulse :type Vector :default "0, 0, 0") (Hit :type Hit%20Result%20Structure%20%28by%20ref%29))
  (bind _returnvalue (Transformation|GetActorLocation))
  ;[1 1 1] Rumble and Fall
  (if (== Other (Game|Player|GetPlayerPawn 0))
    (bind (_direction _newtrack_0 _newtrack_1) (Timeline|Break Play)
      (:Update
        (Transformation|SetActorLocation (Math|Vector|Lerp(Vector) _returnvalue (+ _returnvalue _newtrack_1) _newtrack_0) false false)))))

(fn ConstructionScript)