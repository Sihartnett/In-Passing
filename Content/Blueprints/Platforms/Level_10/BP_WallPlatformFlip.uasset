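; BP_WallPlatformFlip is a Level 10 wall platform actor that spins continuously around its local axes.
; BeginPlay picks roll (X) and pitch (Y) increments from per-axis toggles and amounts, using zero for a disabled axis.
; A looping 0.01-second timer, rather than Tick, adds that local rotation on each call, so the step is not scaled by delta time.
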(event Custom|StartSpinning
  (Utilities|Time|SetTimerbyEvent (delegate Custom|Spin) 0.01 true))

(event Custom|Spin
  (Transformation|AddActorLocalRotation (Math|Rotator|MakeRotator (Variables|Default|GetRotateXToAdd) (Variables|Default|GetRotateYToAdd) 0.0) false false))

(event EventBeginPlay
  (if (Variables|Default|GetRotateY)
    (Variables|Default|SetRotateYToAdd (Variables|Default|GetRotateYAmount))
    (else
      (Variables|Default|SetRotateYToAdd 0.0)))
  (if (Variables|Default|GetRotateX)
    (Variables|Default|SetRotateXToAdd (Variables|Default|GetRotateXAmount))
    (else
      (Variables|Default|SetRotateXToAdd 0.0)))
  (CallFunction|StartSpinning))

(fn ConstructionScript)