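; BP_SmallConveyerPlatform_Child is a Level 10 child variant of a small conveyor platform that reacts to the player touching it.
; When the player pawn overlaps its collision and the platform is not set to start active, it calls MoveTo.
; It resets the move counter first if it sits at its reference start transform and StayOn is false.
; BeginPlay is disabled and construction defers to the parent.
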(event OnComponentBeginOverlap(Collision)
  (params (OverlappedComponent :type Primitive%20Component%20Object%20Reference) (OtherActor :type Actor%20Object%20Reference) (OtherComp :type Primitive%20Component%20Object%20Reference) (OtherBodyIndex :type Integer) (bFromSweep :type Boolean) (SweepResult :type Hit%20Result%20Structure%20%28by%20ref%29))
  (if (and (== OtherActor (Game|Player|GetPlayerPawn 0)) (not (Variables|Default|GetStartsActive)))
    (if (and (== (Transformation|GetActorTransform) (Variables|Default|GetREFStartTransform)) (not (Variables|Default|GetStayOn?)))
      (CallFunction|ResetMoveCounter)
      (else
        (Utilities|FlowControl|DoOnce false
          (:Completed
            _))))
    (CallFunction|Moveto)))

(event EventBeginPlay
  (|CallParentFunction) ; This node is disabled and will not be called.\nDrag off pins to build functionality.
)

(event Collision|EventActorBeginOverlap
  (params (OtherActor :type Actor%20Object%20Reference)))

(event EventTick
  (params (DeltaSeconds :type Float%20%28single-precision%29)))

(fn ConstructionScript
  (|CallParentFunction))