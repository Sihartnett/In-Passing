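; Child Blueprint of a moving conveyor platform that makes the player slippery while inside its Collision volume.
; Entering Collision also starts movement if the platform is idle at its start, not StartsActive or StayOn, resetting the move counter after two moves.
; Entering GroundFrictionCollider subtracts platform velocity from the player's to fix a landing bug.
; It also enables actor input so dummy mouse-button handlers swallow clicks until exit.
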(event OnComponentBeginOverlap(Collision)
  (params (OverlappedComponent :type Primitive%20Component%20Object%20Reference) (OtherActor :type Actor%20Object%20Reference) (OtherComp :type Primitive%20Component%20Object%20Reference) (OtherBodyIndex :type Integer) (bFromSweep :type Boolean) (SweepResult :type Hit%20Result%20Structure%20%28by%20ref%29))
  (bind _returnvalue (Game|Player|GetPlayerPawn 0))
  (if (== OtherActor _returnvalue)
    (Default|SlipperyMovement (.AsFirst%20Person%20Character (Utilities|Casting|CastToFirstPersonCharacter _returnvalue)))
    (if (not (Variables|Default|GetStartsActive))
      (if (and (and (== (Transformation|GetActorTransform) (Variables|Default|GetREFStartTransform)) (not (Variables|Default|GetStayOn?))) (== (Variables|Default|GetTimesMoved) 2))
        (CallFunction|ResetMoveCounter))
      (if (and (== (Transformation|GetActorTransform) (Variables|Default|GetREFStartTransform)) (not (Variables|Default|GetStayOn?)))
        (CallFunction|Moveto)))))

(event OnComponentEndOverlap(Collision)
  (params (OverlappedComponent :type Primitive%20Component%20Object%20Reference) (OtherActor :type Actor%20Object%20Reference) (OtherComp :type Primitive%20Component%20Object%20Reference) (OtherBodyIndex :type Integer))
  (bind _returnvalue (Game|Player|GetPlayerPawn 0))
  (if (== OtherActor _returnvalue)
    (Default|DefaultMovement (.AsFirst%20Person%20Character (Utilities|Casting|CastToFirstPersonCharacter _returnvalue)))))

(event OnComponentEndOverlap(GroundFrictionCollider)
  (params (OverlappedComponent :type Primitive%20Component%20Object%20Reference) (OtherActor :type Actor%20Object%20Reference) (OtherComp :type Primitive%20Component%20Object%20Reference) (OtherBodyIndex :type Integer))
  ;[0.03478 1 0.5326] Platform landing stopping bug
  (if (== OtherActor (Game|Player|GetPlayerPawn 0))
    (Input|DisableInput 0)))

(event OnComponentBeginOverlap(GroundFrictionCollider)
  (params (OverlappedComponent :type Primitive%20Component%20Object%20Reference) (OtherActor :type Actor%20Object%20Reference) (OtherComp :type Primitive%20Component%20Object%20Reference) (OtherBodyIndex :type Integer) (bFromSweep :type Boolean) (SweepResult :type Hit%20Result%20Structure%20%28by%20ref%29))
  (bind _returnvalue (Game|GetPlayerCharacter 0))
  ;[0.03478 1 0.5326] Platform landing stopping bug
  (if (== OtherActor (Game|Player|GetPlayerPawn 0))
    (Input|EnableInput (Game|GetPlayerController 0))
    (bind _returnvalue_2 (Physics|GetPhysicsLinearVelocity (Variables|Default|GetPlatform) "None"))
    (Variables|/Script/Engine.MovementComponent|SetVelocity (Variables|/Script/Engine.Character|GetCharacterMovement _returnvalue) (- (Transformation|GetVelocity _returnvalue) _returnvalue_2))))

(event EventBeginPlay
  (|CallParentFunction) ; This node is disabled and will not be called.\nDrag off pins to build functionality.
)

(event Input|MouseEvents|LeftMouseButton
  (params (Key :type Key%20Structure))
  ;[0.03478 1 0.5326] Platform landing stopping bug
  (:Pressed
    (Variables|Default|SetInputEater "Omae wa mou shindeiru")))

(event Input|MouseEvents|RightMouseButton
  (params (Key :type Key%20Structure))
  ;[0.03478 1 0.5326] Platform landing stopping bug
  (:Pressed
    (Variables|Default|SetInputEater "Oh you thought you could dodge")))

(fn ConstructionScript
  (|CallParentFunction))