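; Platform actor that travels to a target location, triggered the first time the player pawn overlaps its Box.
; MoveTo waits a start delay, then uses MoveComponentTo to move the Platform over a configurable time, with ease flags wired crosswise.
; A Return event delays before triggering that node's Return input, but nothing here calls it.
; An older Timeline-based back-and-forth loop remains disconnected.
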(event OnComponentBeginOverlap(Box)
  (params (OverlappedComponent :type Primitive%20Component%20Object%20Reference) (OtherActor :type Actor%20Object%20Reference) (OtherComp :type Primitive%20Component%20Object%20Reference) (OtherBodyIndex :type Integer) (bFromSweep :type Boolean) (SweepResult :type Hit%20Result%20Structure%20%28by%20ref%29))
  ;[1 1 1] Move Functionality
  (if (== OtherActor (Game|Player|GetPlayerPawn 0))
    (Utilities|FlowControl|DoOnce false
      (:Completed
        (CallFunction|Moveto)))))

(event Custom|MoveTo
  ;[1 1 1] Move Functionality
  (Utilities|FlowControl|Delay (Variables|Default|GetStartWaitTime))
  (Components|MoveComponentTo (Variables|Default|GetPlatform) (Transformation|GetWorldLocation (Variables|Default|GetTargetLocation)) "0, 0, 0" (Variables|Default|GetShouldEaseIn) (Variables|Default|GetShouldEaseOut) (Variables|Default|GetTimeInTransit) false))

(event Custom|StartMoving)

(event Custom|Reverse)

(event Custom|Return
  ;[1 1 1] Move Functionality
  (Utilities|FlowControl|Delay (Variables|Default|GetReturnWaitTime))
  (Components|MoveComponentTo (Variables|Default|GetPlatform) (Transformation|GetWorldLocation (Variables|Default|GetTargetLocation)) "0, 0, 0" (Variables|Default|GetShouldEaseIn) (Variables|Default|GetShouldEaseOut) (Variables|Default|GetTimeInTransit) false) ; enters at Return
)

(fn ConstructionScript)