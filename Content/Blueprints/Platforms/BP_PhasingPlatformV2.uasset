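; Platform whose rock repeatedly phases out and back in, losing and regaining collision as it does.
; After a random start delay, two timelines drive a scalar on a dynamic material instance, toggling collision within set value windows.
; The fade-in timeline restarts the cycle from its update.
; A sphere overlap tracks the player so the phase-in sound, scaled by the GameInstance effects volume, plays only when nearby.
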(event OnComponentBeginOverlap(Sphere)
  (params (OverlappedComponent :type Primitive%20Component%20Object%20Reference) (OtherActor :type Actor%20Object%20Reference) (OtherComp :type Primitive%20Component%20Object%20Reference) (OtherBodyIndex :type Integer) (bFromSweep :type Boolean) (SweepResult :type Hit%20Result%20Structure%20%28by%20ref%29))
  (if (== OtherActor (Game|Player|GetPlayerPawn 0))
    (Variables|Default|SetPlayerInRange true)))

(event OnComponentEndOverlap(Sphere)
  (params (OverlappedComponent :type Primitive%20Component%20Object%20Reference) (OtherActor :type Actor%20Object%20Reference) (OtherComp :type Primitive%20Component%20Object%20Reference) (OtherBodyIndex :type Integer))
  (if (== OtherActor (Game|Player|GetPlayerPawn 0))
    (Variables|Default|SetPlayerInRange false)))

(event Custom|PhasingOut)

(event Custom|PhasingIn)

(event Custom|Lerp%20Platform)

(event Custom|Phasing
  (Utilities|FlowControl|Delay 2.0)
  (bind _newtrack_0 (Timeline|Timeline_1 PlayFromStart)
    (:Update
      (Rendering|Material|SetScalarParameterValue (Variables|Default|GetREFPhasingMaterial) "Yeeter" _newtrack_0 :!class /Script/Engine.MaterialInstanceDynamic)
      (if (Math|Float|InRange(Float) _newtrack_0 0.1 0.49)
        (Collision|SetCollisionEnabled (Variables|Default|GetRock) "NoCollision")))
    (:Finished
      (Utilities|FlowControl|Delay 2.0)
      (if (Variables|Default|GetPlayerInRange)
        (Audio|PlaySoundatLocation "/Game/Audio_Files/Phasing_Platform.Phasing_Platform" "0, 0, 0" "0, 0, 0" (Variables|/Game/Blueprints/BP_GameInstance.BP_GameInstance_C|GetSound%20effects%20volume (Variables|Default|Getref_GameInstance)) 1.0 0.0 0 0 0)
        (bind _newtrack_0_2 (Timeline|Timeline_0 PlayFromStart)
          (:Update
            (Rendering|Material|SetScalarParameterValue (Variables|Default|GetREFPhasingMaterial) "Yeeter" _newtrack_0_2 :!class /Script/Engine.MaterialInstanceDynamic)
            (if (Math|Float|InRange(Float) _newtrack_0_2 0.75 0.8)
              (Collision|SetCollisionEnabled (Variables|Default|GetRock) "QueryAndPhysics")
              (CallFunction|Phasing))))
        (else
          (Timeline|Timeline_0 PlayFromStart))))))

(event EventBeginPlay
  (bind _rock (Variables|Default|GetRock))
  (bind _asbp_game_instance (Utilities|Casting|CastToBP_GameInstance (Game|GetGameInstance)))
  (Variables|Default|Setref_GameInstance _asbp_game_instance)
  (Rendering|Material|SetMaterial _rock 0 "/Game/Assets/Platforms/Materials/M_Platform_Phasing.M_Platform_Phasing")
  (bind _returnvalue (Rendering|Material|CreateDynamicMaterialInstance _rock 0 "/Game/Assets/Platforms/Materials/M_Platform_Phasing.M_Platform_Phasing" "None" :!class /Script/Engine.PrimitiveComponent))
  (Variables|Default|SetREFPhasingMaterial _returnvalue)
  (Utilities|FlowControl|Delay (Math|Random|RandomFloatinRange 0.0 2.0))
  (CallFunction|Phasing))

(fn ConstructionScript)