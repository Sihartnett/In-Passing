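; Rotating pencil platform for Level 5 that spins only while the player pawn overlaps it.
; Begin overlap starts a fast looping timer that adds a set local rotation to the actor on each firing, instead of using Event Tick.
; End overlap clears that timer, stopping the pencil at its current orientation.
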(event Custom|Rotation
  (Transformation|AddActorLocalRotation (Variables|Default|GetRoation%20Amount) false false))

(event Collision|EventActorBeginOverlap
  (params (OtherActor :type Actor%20Object%20Reference))
  (if (== OtherActor (Game|Player|GetPlayerPawn 0))
    (bind _returnvalue (Utilities|Time|SetTimerbyEvent (delegate Custom|Rotation) 0.01 true))))

(event Collision|EventActorEndOverlap
  (params (OtherActor :type Actor%20Object%20Reference))
  (if (== OtherActor (Game|Player|GetPlayerPawn 0))
    (Utilities|Time|ClearandInvalidateTimerbyHandle (stale Collision|EventActorBeginOverlap _returnvalue))))

(fn ConstructionScript)