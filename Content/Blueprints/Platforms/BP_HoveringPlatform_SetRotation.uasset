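; Hovering platform actor that moves back and forth between its start location and an offset while constantly rotating.
; BeginPlay stores the start, subtracts MovementAmount to get the destination, then begins hovering after a PauseTime delay.
; Two timelines drive location lerps without sweep, each starting the other on finish for an endless loop.
; Tick adds RotationRate as local rotation without delta-time scaling, so spin speed depends on frame rate.
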(event Custom|Hover
  (bind _floatlerp (Timeline|Timeline_0 PlayFromStart)
    (:Update
      (Transformation|SetActorLocation (Math|Vector|Lerp(Vector) (Variables|Default|GetREFOriginalLoc) (Variables|Default|GetREFHoverDestination) _floatlerp) false false))
    (:Finished
      (CallFunction|HoverReverse))))

(event Custom|HoverReverse
  (bind _floatlerp (Timeline|Timeline_1 PlayFromStart)
    (:Update
      (Transformation|SetActorLocation (Math|Vector|Lerp(Vector) (Variables|Default|GetREFHoverDestination) (Variables|Default|GetREFOriginalLoc) _floatlerp) false false))
    (:Finished
      (CallFunction|Hover))))

(event EventBeginPlay
  (bind _output_get (Variables|Default|SetREFOriginalLoc (Transformation|GetActorLocation)))
  (Variables|Default|SetREFHoverDestination (- _output_get (Variables|Default|GetMovement%20Amount)))
  (Utilities|FlowControl|Delay (Variables|Default|GetPause%20Time))
  (CallFunction|Hover))

(event EventTick
  (params (DeltaSeconds :type Float%20%28single-precision%29))
  (Transformation|AddActorLocalRotation (Variables|Default|GetRotation%20Rate) false false))

(fn ConstructionScript)