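; Breakable platform that plays a crumbling sound and moves off its spot when the player pawn enters its overlap volume.
; The Break timeline drives that motion by offsetting the actor from its current location each update, so movement accumulates.
; A second timeline continually restarts itself to shake the platform mesh through absolute world rotation.
; ResetPos stops the break and restores the transform saved at BeginPlay, intended for player death.
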(event OnComponentBeginOverlap(BreakOverlap)
  (params (OverlappedComponent :type Primitive%20Component%20Object%20Reference) (OtherActor :type Actor%20Object%20Reference) (OtherComp :type Primitive%20Component%20Object%20Reference) (OtherBodyIndex :type Integer) (bFromSweep :type Boolean) (SweepResult :type Hit%20Result%20Structure%20%28by%20ref%29))
  (bind _returnvalue (Transformation|GetActorLocation))
  ;[1 1 1] Rumble and Fall
  (if (== OtherActor (Game|Player|GetPlayerPawn 0))
    (Audio|PlaySound2D "/Game/Audio_Files/crumbling_platform.crumbling_platform" 1.0 1.0 0.0 0 0)
    (bind (_direction _newtrack_0 _newtrack_1) (Timeline|Break PlayFromStart)
      (:Update
        (Transformation|SetActorLocation (Math|Vector|Lerp(Vector) _returnvalue (+ _returnvalue _newtrack_1) _newtrack_0) false false)))))

(event Custom|StaticShake
  (bind _newtrack_0 (Timeline|Timeline_0 PlayFromStart)
    (:Update
      (Transformation|SetWorldRotation (Variables|Default|GetPlatform) (Math|Rotator|MakeRotator (.x _newtrack_0) (.y _newtrack_0) (.z _newtrack_0)) false false))
    (:Finished
      (CallFunction|StaticShake))))

(event Custom|ResetPos
  (bind _returnvalue (Transformation|GetActorLocation))
  (bind _reftransform (Variables|Default|GetREFTransform))
  ;[1 1 1] Reset On Player Death
  (Transformation|SetActorLocationAndRotation (.location _reftransform) (.rotation _reftransform))
  ;[1 1 1] Rumble and Fall
  (bind (_direction _newtrack_0 _newtrack_1) (Timeline|Break Stop)
    (:Update
      (Transformation|SetActorLocation (Math|Vector|Lerp(Vector) _returnvalue (+ _returnvalue _newtrack_1) _newtrack_0) false false))))

(event EventBeginPlay
  ;[1 1 1] Set Loc Ref
  (Variables|Default|SetREFTransform (Transformation|GetActorTransform))
  (CallFunction|StaticShake))

(event EventTick
  (params (DeltaSeconds :type Float%20%28single-precision%29))
  ;[1 1 1] Set Loc Ref
)

(fn ConstructionScript)