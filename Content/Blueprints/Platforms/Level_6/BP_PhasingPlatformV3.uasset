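; Level 6 platform that repeatedly phases out and back in, toggling its rock mesh's collision as it goes.
; A dynamic material's "Yeeter" scalar is driven by two timelines, with collision switched when the value enters a narrow window.
; Phasing re-triggers itself during phase-in, using separate in and out delays.
; An optional random first delay varies the starting time.
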(event Custom|Phasing
  (if (Variables|Default|GetFirst%20delay)
    (Utilities|FlowControl|Delay (Variables|Default|GetDelay%20First%20Phase))
    (Variables|Default|SetFirst%20delay false)
    (bind _newtrack_0 (Timeline|Timeline_1 PlayFromStart)
      (:Update
        (Rendering|Material|SetScalarParameterValue (Variables|Default|GetREFPhasingMaterial) "Yeeter" _newtrack_0 :!class /Script/Engine.MaterialInstanceDynamic)
        (if (Math|Float|InRange(Float) _newtrack_0 0.2 0.25)
          (Collision|SetCollisionEnabled (Variables|Default|GetRock) "NoCollision")))
      (:Finished
        (Utilities|FlowControl|Delay (Variables|Default|GetPhase%20in%20Delay))
        (bind _newtrack_0_2 (Timeline|Timeline_0 PlayFromStart)
          (:Update
            (Rendering|Material|SetScalarParameterValue (Variables|Default|GetREFPhasingMaterial) "Yeeter" _newtrack_0_2 :!class /Script/Engine.MaterialInstanceDynamic)
            (if (Math|Float|InRange(Float) _newtrack_0_2 0.75 0.8)
              (Collision|SetCollisionEnabled (Variables|Default|GetRock) "QueryAndPhysics")
              (CallFunction|Phasing))))))
    (else
      (Utilities|FlowControl|Delay (Variables|Default|GetPhase%20Out%20Delay))
      (Timeline|Timeline_1 PlayFromStart))))

(event EventBeginPlay
  (bind _rock (Variables|Default|GetRock))
  (Variables|Default|SetFirst%20delay true)
  (Rendering|Material|SetMaterial _rock 0 "/Game/Assets/Platforms/Materials/M_Platform_PhasingWall.M_Platform_PhasingWall")
  (bind _returnvalue (Rendering|Material|CreateDynamicMaterialInstance _rock 0 "/Game/Assets/Platforms/Materials/M_Platform_PhasingWall.M_Platform_PhasingWall" "None" :!class /Script/Engine.PrimitiveComponent))
  (Variables|Default|SetREFPhasingMaterial _returnvalue)
  (if (Variables|Default|GetRandom%20First%20Phase%20Time)
    (Variables|Default|SetDelay%20First%20Phase (Math|Random|RandomFloatinRange 0.0 2.5)))
  (CallFunction|Phasing))

(fn ConstructionScript)