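; BP_IcePlatform is a platform that switches the player to slippery movement while overlapping its Box and restores default movement on exit.
; An ice sound plays at the game instance's SFX volume, then a looping timer steps it down to silence after exit.
; A DashStop volume enables actor input so dummy mouse-button handlers swallow clicks, apparently working around a landing bug that involves dashing.
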(event OnComponentBeginOverlap(Box)
  (params (OverlappedComponent :type Primitive%20Component%20Object%20Reference) (OtherActor :type Actor%20Object%20Reference) (OtherComp :type Primitive%20Component%20Object%20Reference) (OtherBodyIndex :type Integer) (bFromSweep :type Boolean) (SweepResult :type Hit%20Result%20Structure%20%28by%20ref%29))
  (bind _returnvalue (Game|Player|GetPlayerPawn 0))
  (bind _ice_platform_sound_component (Variables|Default|GetIce%20Platform%20Sound%20Component))
  (if (== OtherActor _returnvalue)
    (Audio|Components|Audio|SetVolumeMultiplier _ice_platform_sound_component (Variables|/Game/Blueprints/BP_GameInstance.BP_GameInstance_C|GetSFXVolume (Variables|Default|Getref_GameInstance)) :!class /Script/Engine.AudioComponent)
    (Audio|Components|Audio|Play _ice_platform_sound_component 0.0)
    (Default|SlipperyMovement (.AsFirst%20Person%20Character (Utilities|Casting|CastToFirstPersonCharacter _returnvalue)))))

(event OnComponentEndOverlap(Box)
  (params (OverlappedComponent :type Primitive%20Component%20Object%20Reference) (OtherActor :type Actor%20Object%20Reference) (OtherComp :type Primitive%20Component%20Object%20Reference) (OtherBodyIndex :type Integer))
  (bind _returnvalue (Game|Player|GetPlayerPawn 0))
  (if (== OtherActor _returnvalue)
    (Default|DefaultMovement (.AsFirst%20Person%20Character (Utilities|Casting|CastToFirstPersonCharacter _returnvalue)))
    (bind _returnvalue_2 (Utilities|Time|SetTimerbyEvent (delegate Custom|Fade%20Sound) 0.5 true))))

(event OnComponentBeginOverlap(DashStop)
  (params (OverlappedComponent :type Primitive%20Component%20Object%20Reference) (OtherActor :type Actor%20Object%20Reference) (OtherComp :type Primitive%20Component%20Object%20Reference) (OtherBodyIndex :type Integer) (bFromSweep :type Boolean) (SweepResult :type Hit%20Result%20Structure%20%28by%20ref%29))
  ;[0.03478 1 0.5326] Platform landing stopping bug
  (if (== OtherActor (Game|Player|GetPlayerPawn 0))
    (Input|EnableInput (Game|GetPlayerController 0))))

(event OnComponentEndOverlap(DashStop)
  (params (OverlappedComponent :type Primitive%20Component%20Object%20Reference) (OtherActor :type Actor%20Object%20Reference) (OtherComp :type Primitive%20Component%20Object%20Reference) (OtherBodyIndex :type Integer))
  ;[0.03478 1 0.5326] Platform landing stopping bug
  (if (== OtherActor (Game|Player|GetPlayerPawn 0))
    (Input|DisableInput 0)))

(event Custom|Fade%20Sound
  (bind _ice_platform_sound_component (Variables|Default|GetIce%20Platform%20Sound%20Component))
  (Math|Float|CompareFloat (Variables|/Script/Engine.AudioComponent|GetVolumeMultiplier _ice_platform_sound_component) 0.0
    (:>
      (Audio|Components|Audio|SetVolumeMultiplier (Variables|Default|GetIce%20Platform%20Sound%20Component) (- (Variables|/Script/Engine.AudioComponent|GetVolumeMultiplier (Variables|Default|GetIce%20Platform%20Sound%20Component)) 0.5) :!class /Script/Engine.AudioComponent))
    (:==
      (Audio|Components|Audio|Stop _ice_platform_sound_component :!label _label)
      (Utilities|Time|ClearandInvalidateTimerbyHandle (stale OnComponentEndOverlap(Box) _returnvalue_2)))
    (:<
      (goto _label))))

(event EventBeginPlay
  (Audio|Components|Audio|SetSound (Variables|Default|GetIce%20Platform%20Sound%20Component) "/Game/Audio_Files/Sound_Cues/Ice_platform_Cue.Ice_platform_Cue")
  (bind _asbp_game_instance (Utilities|Casting|CastToBP_GameInstance (Game|GetGameInstance)))
  (Variables|Default|Setref_GameInstance _asbp_game_instance))

(event EventTick
  (params (DeltaSeconds :type Float%20%28single-precision%29)))

(event Input|MouseEvents|LeftMouseButton
  (params (Key :type Key%20Structure))
  ;[0.03478 1 0.5326] Platform landing stopping bug
  (:Pressed
    (Variables|Default|SetInputEater "Omae wa mou shindeiru")))

(event Input|MouseEvents|RightMouseButton
  (params (Key :type Key%20Structure))
  ;[0.03478 1 0.5326] Platform landing stopping bug
  (:Pressed
    (Variables|Default|SetInputEater "Oh you thought you could dodge")))

(fn ConstructionScript)