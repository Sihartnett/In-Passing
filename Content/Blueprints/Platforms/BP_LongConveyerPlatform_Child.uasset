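; BP_LongConveyerPlatform_Child is a child Blueprint of a conveyor platform that changes how the first-person player moves while on it.
; When the player pawn enters its Collision volume it switches the character to slippery movement, and leaving restores default movement.
; If the platform does not start active, the first player overlap also calls MoveTo once, through a DoOnce.
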(event OnComponentBeginOverlap(Collision)
  (params (OverlappedComponent :type Primitive%20Component%20Object%20Reference) (OtherActor :type Actor%20Object%20Reference) (OtherComp :type Primitive%20Component%20Object%20Reference) (OtherBodyIndex :type Integer) (bFromSweep :type Boolean) (SweepResult :type Hit%20Result%20Structure%20%28by%20ref%29))
  (bind _returnvalue (Game|Player|GetPlayerPawn 0))
  (if (== OtherActor _returnvalue)
    (Default|SlipperyMovement (.AsFirst%20Person%20Character (Utilities|Casting|CastToFirstPersonCharacter _returnvalue)))
    (if (not (Variables|Default|GetStartsActive))
      (Utilities|FlowControl|DoOnce false
        (:Completed
          (CallFunction|Moveto))))))

(event OnComponentEndOverlap(Collision)
  (params (OverlappedComponent :type Primitive%20Component%20Object%20Reference) (OtherActor :type Actor%20Object%20Reference) (OtherComp :type Primitive%20Component%20Object%20Reference) (OtherBodyIndex :type Integer))
  (bind _returnvalue (Game|Player|GetPlayerPawn 0))
  (if (== OtherActor _returnvalue)
    (Default|DefaultMovement (.AsFirst%20Person%20Character (Utilities|Casting|CastToFirstPersonCharacter _returnvalue)))))

(event EventBeginPlay
  (|CallParentFunction) ; This node is disabled and will not be called.\nDrag off pins to build functionality.
)

(event Collision|EventActorBeginOverlap
  (params (OtherActor :type Actor%20Object%20Reference)))

(event EventTick
  (params (DeltaSeconds :type Float%20%28single-precision%29)))

(fn ConstructionScript
  (|CallParentFunction))