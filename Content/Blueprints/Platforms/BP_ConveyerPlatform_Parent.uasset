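; Parent Blueprint for a conveyer platform that shuttles its Platform component between the actor's starting transform and TargetLocation.
; MoveTo waits StartWaitTime, runs MoveComponentTo with optional easing, flips the Returning flag, then calls itself again.
; StartsActive sets StayOn at BeginPlay for endless looping; without StayOn, TimesMoved limits a triggered MoveTo to one round trip until ResetMoveCounter clears it.
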(event Custom|MoveTo
  ;[1 1 1] Move Functionality
  (Utilities|FlowControl|Delay (Variables|Default|GetStartWaitTime))
  (if (Variables|Default|GetStayOn?)
    (Components|MoveComponentTo (Variables|Default|GetPlatform) (.location (select (Variables|Default|GetReturning?) (Variables|Default|GetREFStartTransform) (Transformation|GetWorldTransform (Variables|Default|GetTargetLocation)))) (.rotation (select (Variables|Default|GetReturning?) (Variables|Default|GetREFStartTransform) (Transformation|GetWorldTransform (Variables|Default|GetTargetLocation)))) (Variables|Default|GetShouldEaseIn) (Variables|Default|GetShouldEaseOut) (Variables|Default|GetTimeInTransit) false :!label _label)
    (Utilities|FlowControl|FlipFlop
      (:A
        (Variables|Default|SetReturning? true))
      (:B
        (Variables|Default|SetReturning? false)))
    (Math|Integer|IncrementInt (Variables|Default|GetTimesMoved)
      (:%20%20
        (CallFunction|Moveto)))
    (elif (<= (Variables|Default|GetTimesMoved) 1)
      (goto _label))))

(event Custom|ResetMoveCounter
  (Variables|Default|SetTimesMoved 0))

(event Custom|ResetDoOnce)

(event EventBeginPlay
  (Variables|Default|SetREFStartTransform (Transformation|GetActorTransform))
  (if (Variables|Default|GetStartsActive)
    (Variables|Default|SetStayOn? true)
    (CallFunction|Moveto)))

(fn ConstructionScript)