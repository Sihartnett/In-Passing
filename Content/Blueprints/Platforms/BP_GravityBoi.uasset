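; BP_GravityBoi is a gravity platform actor that pulls the player pawn toward its Sphere component.
; Any overlap with GravityZone toggles an in-range flag, without checking the overlapping actor, and Tick calls PullPlayer while it is set.
; PullPlayer adds velocity toward the sphere, weighted more heavily vertically and scaled up with the player's speed within a clamped range.
; The pull applies per frame, without delta-time scaling.
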(event OnComponentBeginOverlap(GravityZone)
  (params (OverlappedComponent :type Primitive%20Component%20Object%20Reference) (OtherActor :type Actor%20Object%20Reference) (OtherComp :type Primitive%20Component%20Object%20Reference) (OtherBodyIndex :type Integer) (bFromSweep :type Boolean) (SweepResult :type Hit%20Result%20Structure%20%28by%20ref%29))
  (Variables|Default|SetPlayerinRange true))

(event OnComponentEndOverlap(GravityZone)
  (params (OverlappedComponent :type Primitive%20Component%20Object%20Reference) (OtherActor :type Actor%20Object%20Reference) (OtherComp :type Primitive%20Component%20Object%20Reference) (OtherBodyIndex :type Integer))
  (Variables|Default|SetPlayerinRange false))

(event Custom|PullPlayer
  (bind _returnvalue (Game|Player|GetPlayerPawn 0))
  (bind _sphere (Variables|Default|GetSphere))
  (bind _returnvalue_2 (Pawn|GetMovementComponent _returnvalue))
  (bind _returnvalue_3 (Transformation|GetActorLocation _returnvalue))
  (bind _returnvalue_4 (Transformation|GetWorldLocation _sphere))
  (bind _returnvalue_5 (- _returnvalue_4 _returnvalue_3))
  (bind _returnvalue_6 (Math|Vector|Normalize _returnvalue_5))
  (Variables|/Script/Engine.MovementComponent|SetVelocity _returnvalue_2 (+ (Math|Vector|MakeVector (* (Math|Float|MapRangeClamped (Math|Vector|VectorLength (Variables|/Script/Engine.MovementComponent|GetVelocity _returnvalue_2)) 8e+02 4e+03 1.0 4.0) (* (.x _returnvalue_6) 8.0)) (* (Math|Float|MapRangeClamped (Math|Vector|VectorLength (Variables|/Script/Engine.MovementComponent|GetVelocity _returnvalue_2)) 8e+02 4e+03 1.0 4.0) (* (.y _returnvalue_6) 8.0)) (* (Math|Float|MapRangeClamped (Math|Vector|VectorLength (Variables|/Script/Engine.MovementComponent|GetVelocity _returnvalue_2)) 8e+02 4e+03 1.0 4.0) (* (.z _returnvalue_6) 25.0))) (Variables|/Script/Engine.MovementComponent|GetVelocity _returnvalue_2))))

(event EventBeginPlay)

(event Collision|EventActorBeginOverlap
  (params (OtherActor :type Actor%20Object%20Reference)))

(event EventTick
  (params (DeltaSeconds :type Float%20%28single-precision%29))
  (if (Variables|Default|GetPlayerinRange)
    (CallFunction|PullPlayer)))

(fn ConstructionScript)