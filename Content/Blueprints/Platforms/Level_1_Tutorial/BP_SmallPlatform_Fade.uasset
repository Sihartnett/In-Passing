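; Small platform Blueprint for the tutorial level that fades in when its FadeIn event is called.
; BeginPlay creates a dynamic material instance from the mesh's first material and zeroes its "Yeeter" scalar parameter.
; FadeIn enables query and physics collision, then plays the FadingIn timeline from the start to drive that parameter.
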(event Custom|FadeIn
  (Collision|SetCollisionEnabled (Variables|Default|GetStaticMesh) "QueryAndPhysics")
  (bind _newtrack_0 (Timeline|FadingIn PlayFromStart)
    (:Update
      (Rendering|Material|SetScalarParameterValue (Variables|Default|GetREFMaterialInstance) "Yeeter" _newtrack_0 :!class /Script/Engine.MaterialInstanceDynamic))))

(event EventBeginPlay
  (bind _staticmesh (Variables|Default|GetStaticMesh))
  (bind _returnvalue (Rendering|Material|CreateDynamicMaterialInstance _staticmesh 0 (Rendering|Material|GetMaterial _staticmesh 0) "None" :!class /Script/Engine.PrimitiveComponent))
  (bind _output_get (Variables|Default|SetREFMaterialInstance _returnvalue))
  (Rendering|Material|SetScalarParameterValue _output_get "Yeeter" 0.0 :!class /Script/Engine.MaterialInstanceDynamic))

(fn ConstructionScript)