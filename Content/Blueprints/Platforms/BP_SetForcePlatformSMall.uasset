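; Small launch platform that throws the player with a set X/Y/Z velocity on overlap, optionally adding the player's current horizontal velocity.
; The cylinder trigger plays a volume-scaled sound, launches the character, then fires BouncePulse for sparks and a GameMode fade call.
; Timelines drive Emission on a dynamic material created at BeginPlay.
; The looping idle pulse starts only after a bounce flash finishes, as its other call is unwired.
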(event OnComponentBeginOverlap(Cylinder)
  (params (OverlappedComponent :type Primitive%20Component%20Object%20Reference) (OtherActor :type Actor%20Object%20Reference) (OtherComp :type Primitive%20Component%20Object%20Reference) (OtherBodyIndex :type Integer) (bFromSweep :type Boolean) (SweepResult :type Hit%20Result%20Structure%20%28by%20ref%29))
  (bind _returnvalue (Game|GetPlayerCharacter 0))
  (bind _returnvalue_2 (Game|Player|GetPlayerPawn 0))
  (bind _xvelocity (Variables|Default|GetXVelocity))
  (bind _yvelocity (Variables|Default|GetYVelocity))
  (bind _zvelocity (Variables|Default|GetZVelocity))
  (bind _returnvalue_3 (Transformation|GetVelocity _returnvalue_2))
  (bind _returnvalue_4 (Math|Vector|MakeVector _xvelocity _yvelocity _zvelocity))
  (bind _returnvalue_5 (Math|Vector|MakeVector (.x _returnvalue_3) (.y _returnvalue_3) 0.0))
  (bind _returnvalue_6 (+ _returnvalue_4 _returnvalue_5))
  (if (== OtherActor _returnvalue_2)
    (Audio|PlaySound2D "/Game/Audio_Files/Platforms/ChargedPlatform.ChargedPlatform" (Variables|/Game/Blueprints/BP_GameInstance.BP_GameInstance_C|GetSFXVolume (Variables|Default|Getref_GameInstance)) 1.0 0.0 0 0)
    (if (Variables|Default|GetVelocity%20Override)
      (Character|LaunchCharacter _returnvalue (Math|Vector|MakeVector (Variables|Default|GetXVelocity) (Variables|Default|GetYVelocity) (Variables|Default|GetZVelocity)) true true)
      (CallFunction|BouncePulse)
      (else
        (Character|LaunchCharacter _returnvalue (Math|Vector|MakeVector (.x _returnvalue_6) (.y _returnvalue_6) (.z _returnvalue_6)) true true)
        (CallFunction|BouncePulse)))))

(event Custom|IdlePulse
  (bind _pulse (Timeline|PulseTimeline PlayFromStart)
    (:Update
      (Rendering|Material|SetScalarParameterValue (Variables|Default|GetREFMaterial) "Emission" _pulse :!class /Script/Engine.MaterialInstanceDynamic))
    (:Finished
      (CallFunction|IdlePulse))))

(event Custom|BouncePulse
  (CallFunction|IdlePause)
  (CallFunction|SparkParticle)
  (Default|ChargedPlatformFade (.AsBP%20Game%20Mode (Utilities|Casting|CastToBP_GameMode (Game|GetGameMode))))
  (bind _newtrack_0 (Timeline|BouncePulseTimeline PlayFromStart)
    (:Update
      (Rendering|Material|SetScalarParameterValue (Variables|Default|GetREFMaterial) "Emission" _newtrack_0 :!class /Script/Engine.MaterialInstanceDynamic))
    (:Finished
      (CallFunction|IdlePulse))))

(event Custom|IdlePause
  (bind _pulse (Timeline|PulseTimeline Stop)
    (:Update
      (Rendering|Material|SetScalarParameterValue (Variables|Default|GetREFMaterial) "Emission" _pulse :!class /Script/Engine.MaterialInstanceDynamic))
    (:Finished
      (CallFunction|IdlePulse))))

(event EventBeginPlay
  (bind _platform (Variables|Default|GetPlatform))
  (bind _asbp_game_instance (Utilities|Casting|CastToBP_GameInstance (Game|GetGameInstance)))
  (Variables|Default|Setref_GameInstance _asbp_game_instance)
  (Rendering|Material|SetMaterial _platform 0 "/Game/Assets/Platforms/Materials/M_Platform_S1E.M_Platform_S1E")
  (bind _returnvalue (Rendering|Material|CreateDynamicMaterialInstance _platform 0 "/Game/Assets/Platforms/Materials/M_Platform_S1E.M_Platform_S1E" "None" :!class /Script/Engine.PrimitiveComponent))
  (Variables|Default|SetREFMaterial _returnvalue))

(fn ConstructionScript)

(fn SparkParticle
  (Effects|SpawnEmitteratLocation "/Game/Particles/P_Sparks.P_Sparks" (Transformation|GetWorldLocation (Variables|Default|GetSparkSpawnLoc)) "0, 0, 0" (Transformation|GetWorldScale (Variables|Default|GetPlatform))))