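; BP_ChargedPlatform1_small is a small charged bounce platform that launches the player when they overlap its cylinder.
; Launch velocity follows the ForceDirection component's forward vector, scaled by Z velocity, platform world scale and a size multiplier, overriding existing velocity.
; Each launch plays a volume-scaled sound, spawns sparks, notifies BP_GameMode to run its platform fade and pulses a dynamic material's emission via a timeline.
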(event OnComponentBeginOverlap(Cylinder)
  (params (OverlappedComponent :type Primitive%20Component%20Object%20Reference) (OtherActor :type Actor%20Object%20Reference) (OtherComp :type Primitive%20Component%20Object%20Reference) (OtherBodyIndex :type Integer) (bFromSweep :type Boolean) (SweepResult :type Hit%20Result%20Structure%20%28by%20ref%29))
  (if (== OtherActor (Game|Player|GetPlayerPawn 0))
    (Audio|PlaySound2D "/Game/Audio_Files/Platforms/ChargedPlatform.ChargedPlatform" (Variables|/Game/Blueprints/BP_GameInstance.BP_GameInstance_C|GetSFXVolume (Variables|Default|Getref_GameInstance)) 1.0 0.0 0 0)
    (Character|LaunchCharacter (Game|GetPlayerCharacter 0) (* (* (* (Math|Vector|GetForwardVector (Variables|Default|GetForceDirection)) (Variables|Default|GetZVelocity)) (Transformation|GetWorldScale (Variables|Default|GetPlatform))) (Variables|Default|GetSizeVelocityMultiplier)) true true)
    (CallFunction|BouncePulse)))

(event Custom|BouncePulse
  (CallFunction|SparkParticle)
  (Default|ChargedPlatformFade (.AsBP%20Game%20Mode (Utilities|Casting|CastToBP_GameMode (Game|GetGameMode))))
  (bind _newtrack_0 (Timeline|BouncePulseTimeline PlayFromStart)
    (:Update
      (Rendering|Material|SetScalarParameterValue (Variables|Default|GetREFMaterial) "Emission" _newtrack_0 :!class /Script/Engine.MaterialInstanceDynamic))))

(event EventBeginPlay
  (bind _platform (Variables|Default|GetPlatform))
  (bind _asbp_game_instance (Utilities|Casting|CastToBP_GameInstance (Game|GetGameInstance)))
  (Variables|Default|Setref_GameInstance _asbp_game_instance)
  (Rendering|Material|SetMaterial _platform 0 "/Game/Assets/Platforms/Materials/M_Platform_S1E.M_Platform_S1E")
  (bind _returnvalue (Rendering|Material|CreateDynamicMaterialInstance _platform 0 "/Game/Assets/Platforms/Materials/M_Platform_S1E.M_Platform_S1E" "None" :!class /Script/Engine.PrimitiveComponent))
  (Variables|Default|SetREFMaterial _returnvalue))

(fn ConstructionScript)

(fn SparkParticle
  (Effects|SpawnEmitteratLocation "/Game/Particles/P_Sparks.P_Sparks" (Transformation|GetWorldLocation (Variables|Default|GetSparkSpawnLoc)) "0, 0, 0" (Transformation|GetWorldScale (Variables|Default|GetPlatform))))