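; Falling rock platform that collapses a second after the player pawn overlaps its collision while it is active.
; From BeginPlay, a looping timer jitters six rocks with small random rotations and steadily turns a seventh.
; The collapse stops that timer, enables physics on the rocks and disables the Cylinder's collision.
; ResetPos restores the transforms cached at BeginPlay and the collision, re-arms the platform and restarts the shake.
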(event OnComponentBeginOverlap(Collision)
  (params (OverlappedComponent :type Primitive%20Component%20Object%20Reference) (OtherActor :type Actor%20Object%20Reference) (OtherComp :type Primitive%20Component%20Object%20Reference) (OtherBodyIndex :type Integer) (bFromSweep :type Boolean) (SweepResult :type Hit%20Result%20Structure%20%28by%20ref%29))
  ;[1 1 1] Rock Physics
  (if (and (== OtherActor (Game|Player|GetPlayerPawn 0)) (Variables|Default|GetisActive))
    (Utilities|FlowControl|Delay 1.0)
    (Utilities|Time|ClearandInvalidateTimerbyHandle (stale Custom|StartShake _returnvalue))
    (CallFunction|RockPhysics)))

(event Custom|ResetPos
  ;[1 1 1] Reset Rocks
  (CallFunction|ResetRocks)
  (CallFunction|StartShake))

(event Custom|StartShake
  (bind _returnvalue (Utilities|Time|SetTimerbyEvent (delegate Custom|Shake) 0.05 true)))

(event Custom|Shake
  (bind _defaultsceneroot (Variables|Default|GetDefaultSceneRoot))
  (bind _returnvalue (Transformation|GetWorldRotation _defaultsceneroot))
  (Transformation|AddLocalRotation (Variables|Default|GetRock1) (Math|Rotator|MakeRotator (Math|Float|Clamp(Float) (+ (.roll _returnvalue) (Math|Random|RandomFloatinRange -0.7 0.7)) -3.5 3.5) (Math|Float|Clamp(Float) (+ (.pitch _returnvalue) (Math|Random|RandomFloatinRange -0.7 0.7)) -3.5 3.5) 0.0) false false)
  (Transformation|AddLocalRotation (Variables|Default|GetRock6) (Math|Rotator|MakeRotator 1.0 -0.5 0.0) false false))

(event EventBeginPlay
  ;[1 1 1] Refs
  (CallFunction|RockRefs)
  (CallFunction|StartShake))

(fn ConstructionScript)

(fn RockRefs
  (Variables|Default|SetRock1Transform (Transformation|GetWorldTransform (Variables|Default|GetRock1)))
  (Variables|Default|SetRock2Transform (Transformation|GetWorldTransform (Variables|Default|GetRock2)))
  (Variables|Default|SetRock3Transform (Transformation|GetWorldTransform (Variables|Default|GetRock3)))
  (Variables|Default|SetRock4Transform (Transformation|GetWorldTransform (Variables|Default|GetRock4)))
  (Variables|Default|SetRock5Transform (Transformation|GetWorldTransform (Variables|Default|GetRock5)))
  (Variables|Default|SetRock6Transform (Transformation|GetWorldTransform (Variables|Default|GetRock)))
  (Variables|Default|SetRock7Transform (Transformation|GetWorldTransform (Variables|Default|GetRock6))))

(fn ResetRocks
  (Physics|SetSimulatePhysics (Variables|Default|GetRock) false)
  (Collision|SetCollisionEnabled (Variables|Default|GetCylinder) "QueryAndPhysics")
  (Transformation|SetWorldTransform (Variables|Default|GetRock1) (Variables|Default|GetRock1Transform) false false)
  (Transformation|SetWorldTransform (Variables|Default|GetRock2) (Variables|Default|GetRock2Transform) false false)
  (Transformation|SetWorldTransform (Variables|Default|GetRock3) (Variables|Default|GetRock3Transform) false false)
  (Transformation|SetWorldTransform (Variables|Default|GetRock4) (Variables|Default|GetRock4Transform) false false)
  (Transformation|SetWorldTransform (Variables|Default|GetRock5) (Variables|Default|GetRock5Transform) false false)
  (Transformation|SetWorldTransform (Variables|Default|GetRock) (Variables|Default|GetRock6Transform) false false)
  (Transformation|SetWorldTransform (Variables|Default|GetRock6) (Variables|Default|GetRock7Transform) false false)
  (Variables|Default|SetisActive true)
  (return))

(fn RockPhysics
  (Physics|SetSimulatePhysics (Variables|Default|GetRock) true)
  (Collision|SetCollisionEnabled (Variables|Default|GetCylinder) "NoCollision")
  (Variables|Default|SetisActive false))