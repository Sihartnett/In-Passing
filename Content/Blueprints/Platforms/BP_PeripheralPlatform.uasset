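; BP_PeripheralPlatform is a rock platform set up to fade through its material as the player enters or leaves a range.
; BeginPlay creates a dynamic material and scales the FadeRange trigger by PeripheralRange.
; Overlaps play timelines that lerp the "Yeeter" scalar toward FinalResultNeeded or 1.0, but Alpha is fixed at zero, so the value stays unchanged.
; Tick stores a player-to-platform look-at rotation that this graph never applies.
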(event OnComponentBeginOverlap(FadeRange)
  (params (OverlappedComponent :type Primitive%20Component%20Object%20Reference) (OtherActor :type Actor%20Object%20Reference) (OtherComp :type Primitive%20Component%20Object%20Reference) (OtherBodyIndex :type Integer) (bFromSweep :type Boolean) (SweepResult :type Hit%20Result%20Structure%20%28by%20ref%29))
  (if (== OtherActor (Game|Player|GetPlayerPawn 0))
    (bind _returnvalue (Rendering|Material|GetScalarParameterValue (Variables|Default|GetREFMaterial) "Yeeter" :!class /Script/Engine.MaterialInstanceDynamic))
    (Variables|Default|SetREFScalarParameter _returnvalue)
    (Timeline|Timeline_0 PlayFromStart
      (:Update
        (Rendering|Material|SetScalarParameterValue (Variables|Default|GetREFMaterial) "Yeeter" (Math|Float|Lerp (Variables|Default|GetREFScalarParameter) (Variables|Default|GetfinalResultNeeded) 0.0) :!class /Script/Engine.MaterialInstanceDynamic)))))

(event OnComponentEndOverlap(FadeRange)
  (params (OverlappedComponent :type Primitive%20Component%20Object%20Reference) (OtherActor :type Actor%20Object%20Reference) (OtherComp :type Primitive%20Component%20Object%20Reference) (OtherBodyIndex :type Integer))
  (if (== OtherActor (Game|Player|GetPlayerPawn 0))
    (bind _returnvalue (Rendering|Material|GetScalarParameterValue (Variables|Default|GetREFMaterial) "Yeeter" :!class /Script/Engine.MaterialInstanceDynamic))
    (Variables|Default|SetREFScalarParameter _returnvalue)
    (Timeline|Timeline_1 PlayFromStart
      (:Update
        (Rendering|Material|SetScalarParameterValue (Variables|Default|GetREFMaterial) "Yeeter" (Math|Float|Lerp (Variables|Default|GetREFScalarParameter) 1.0 0.0) :!class /Script/Engine.MaterialInstanceDynamic)))))

(event EventBeginPlay
  (bind _rock (Variables|Default|GetRock))
  (Variables|Default|SetplatformRotation (Transformation|GetWorldRotation (Variables|Default|GetDefaultSceneRoot)))
  (Rendering|Material|SetMaterial _rock 0 "/Game/Assets/Platforms/Materials/M_Platform_Peripheral.M_Platform_Peripheral")
  (bind _returnvalue (Rendering|Material|CreateDynamicMaterialInstance _rock 0 "/Game/Assets/Platforms/Materials/M_Platform_Peripheral.M_Platform_Peripheral" "None" :!class /Script/Engine.PrimitiveComponent))
  (Variables|Default|SetREFMaterial _returnvalue)
  (Transformation|SetWorldScale3D (Variables|Default|GetFadeRange) (Variables|Default|GetPeripheralRange)))

(event EventTick
  (params (DeltaSeconds :type Float%20%28single-precision%29))
  (Variables|Default|SetplatformRotation (Math|Rotator|FindLookatRotation (Transformation|GetWorldLocation (Variables|/Script/Engine.Actor|GetRootComponent (Game|Player|GetPlayerPawn 0))) (Transformation|GetWorldLocation (Variables|Default|GetDefaultSceneRoot)))))

(fn ConstructionScript)