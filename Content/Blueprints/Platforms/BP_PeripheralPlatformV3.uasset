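; Platform whose rock material responds to the player's peripheral view, with a visibility value that rises as the pawn faces away from it.
; Once the player pawn enters the sphere, Tick maps the pawn's facing dot product, scales it and feeds the dynamic material's "Yeeter" parameter.
; The in-range flag is never cleared, and two timeline fades for the parameter are left unconnected.
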(event OnComponentBeginOverlap(Sphere)
  (params (OverlappedComponent :type Primitive%20Component%20Object%20Reference) (OtherActor :type Actor%20Object%20Reference) (OtherComp :type Primitive%20Component%20Object%20Reference) (OtherBodyIndex :type Integer) (bFromSweep :type Boolean) (SweepResult :type Hit%20Result%20Structure%20%28by%20ref%29))
  (if (== OtherActor (Game|Player|GetPlayerPawn 0))
    (Variables|Default|SetPlayerInRange true)))

(event EventBeginPlay
  (bind _rock (Variables|Default|GetRock))
  (Rendering|Material|SetMaterial _rock 0 "/Game/Assets/Platforms/Materials/M_Platform_Peripheral.M_Platform_Peripheral")
  (bind _returnvalue (Rendering|Material|CreateDynamicMaterialInstance _rock 0 "/Game/Assets/Platforms/Materials/M_Platform_Peripheral.M_Platform_Peripheral" "None" :!class /Script/Engine.PrimitiveComponent))
  (Variables|Default|SetREFRockMaterial _returnvalue))

(event EventTick
  (params (DeltaSeconds :type Float%20%28single-precision%29))
  (if (Variables|Default|GetPlayerInRange)
    (bind _output_get (Variables|Default|SetVisibilityValue (* (Math|Float|MapRangeClamped (Class|Actor|GetDotProductto (Game|Player|GetPlayerPawn 0) self) 1.0 0.0 0.0 1.0) 3.0)))
    (Rendering|Material|SetScalarParameterValue (Variables|Default|GetREFRockMaterial) "Yeeter" _output_get :!class /Script/Engine.MaterialInstanceDynamic)))

(fn ConstructionScript)