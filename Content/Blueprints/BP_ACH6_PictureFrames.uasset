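; Trigger actor that counts the picture frames the player visits toward the LOOK_PHOTOGRAPH achievement.
; The first player-pawn overlap with its Box increments NumberOfPictures on BP_GameMode, with a DoOnce preventing repeat counts from the same instance.
; When the shared count reaches 21, it caches achievements and, on success, writes the achievement progress.
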(event OnComponentBeginOverlap(Box)
  (params (OverlappedComponent :type Primitive%20Component%20Object%20Reference) (OtherActor :type Actor%20Object%20Reference) (OtherComp :type Primitive%20Component%20Object%20Reference) (OtherBodyIndex :type Integer) (bFromSweep :type Boolean) (SweepResult :type Hit%20Result%20Structure%20%28by%20ref%29))
  (bind _returnvalue (Game|GetPlayerController 0))
  (if (== OtherActor (Game|Player|GetPlayerPawn 0))
    (Utilities|FlowControl|DoOnce false
      (:Completed
        (bind _asbp_game_mode (Utilities|Casting|CastToBP_GameMode (Game|GetGameMode)))
        (bind _result (Math|Integer|IncrementInt (Variables|/Game/Blueprints/BP_GameMode.BP_GameMode_C|GetNumberOfPictures _asbp_game_mode))
          (:%20%20
            (if (== _result 21)
              (|CacheAchievements _returnvalue
                (:OnSuccess
                  (|WriteAchievementProgress _returnvalue "LOOK_PHOTOGRAPH" 1e+02))))))))))

(event EventBeginPlay)

(event Collision|EventActorBeginOverlap
  (params (OtherActor :type Actor%20Object%20Reference)))

(event EventTick
  (params (DeltaSeconds :type Float%20%28single-precision%29)))

(fn ConstructionScript)