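; BP_DeathVolume is a moving kill volume that handles player death on overlap.
; Overlap shows a death fade, waits briefly, resets the volume to its start, calls GameMode PlayerDeath, restores the character and increments the GameInstance death count.
; Unless frozen, Tick uses distance and below-player checks to step the volume upward or move it far beneath the player.
; Older respawn and breaking-platform reset logic is left unconnected.
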(event EventBeginPlay
  ;[1 1 1] Set Refs
  (bind _asbp_game_mode (Utilities|Casting|CastToBP_GameMode (Game|GetGameMode)))
  (Variables|Default|SetREFGameMode _asbp_game_mode)
  (bind _asbp_game_instance (Utilities|Casting|CastToBP_GameInstance (Game|GetGameInstance))
    (:then
      (Variables|Default|SetREFGameInstance _asbp_game_instance)
      (Variables|Default|SetRefDeathLoc (Transformation|GetActorLocation))
      (bind _asfirst_person_character (Utilities|Casting|CastToFirstPersonCharacter (Game|Player|GetPlayerPawn 0)))
      (Variables|Default|SetCharacter%20reference _asfirst_person_character))
    (:CastFailed
      (Development|PrintString "No Cast to BP_GameInstance"))))

(event Collision|EventActorBeginOverlap
  (params (OtherActor :type Actor%20Object%20Reference))
  (bind _refgameinstance (Variables|Default|GetREFGameInstance))
  (bind _character_reference (Variables|Default|GetCharacter%20reference))
  ;[1 1 1] Set Player Loc
  (if (== OtherActor (Game|Player|GetPlayerPawn 0))
    (bind _returnvalue (UserInterface|CreateWidget "/Game/Widgets/W_DeathFade.W_DeathFade_C" (Game|GetPlayerController 0)))
    (UserInterface|Viewport|AddtoViewport _returnvalue 0)
    (Utilities|FlowControl|Delay 0.5)
    (Transformation|SetActorLocation (Variables|Default|GetRefDeathLoc) false false)
    (Default|PlayerDeath (Variables|Default|GetREFGameMode))
    (Variables|/Script/Unbelievable.UnbelievableCharacter|SettimeSpentInAir _character_reference 0.0)
    (Default|RestoretoFullHealth _character_reference)
    (Variables|/Game/Blueprints/BP_GameInstance.BP_GameInstance_C|SetNumberOfDeaths _refgameinstance (+ (Variables|/Game/Blueprints/BP_GameInstance.BP_GameInstance_C|GetNumberOfDeaths _refgameinstance) 1))
    (Development|PrintString (Utilities|String|Append "Total Number of Deaths are : " (Utilities|String|ToString(Integer) (+ (Variables|/Game/Blueprints/BP_GameInstance.BP_GameInstance_C|GetNumberOfDeaths _refgameinstance) 1))))))

(event EventTick
  (params (DeltaSeconds :type Float%20%28single-precision%29))
  (bind _returnvalue (Game|Player|GetPlayerPawn 0))
  (bind _returnvalue_2 (Transformation|GetActorLocation))
  (bind _returnvalue_3 (Transformation|GetActorLocation _returnvalue))
  ;[1 1 1] Move Death Volume
  (if (not (Variables|Default|GetFreeze%20death%20Volume))
    (if (|DistanceCheck)
      (Transformation|SetActorLocation (Math|Vector|MakeVector (.x _returnvalue_2) (.y _returnvalue_2) (+ (.z _returnvalue_2) 1e+02)) false false)
      (elif (|Checkisplayerisasbelow)
        (Transformation|SetActorLocation (Math|Vector|MakeVector (.x _returnvalue_3) (.y _returnvalue_3) (- (.z _returnvalue_3) 5e+04)) false false)))))

(fn ConstructionScript)