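; BP_LampTree_Vignette is a lamp prop that swings on its roll axis while the player pawn is inside its StartSwingingVolume.
; Overlap starts a fast looping timer after a short random delay, and leaving the volume clears it.
; Each tick adds a step to the lamp's world roll, zeroing pitch and yaw.
; The step changes direction and size at positive and negative limits randomized on BeginPlay.
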(event OnComponentBeginOverlap(StartSwingingVolume)
  (params (OverlappedComponent :type Primitive%20Component%20Object%20Reference) (OtherActor :type Actor%20Object%20Reference) (OtherComp :type Primitive%20Component%20Object%20Reference) (OtherBodyIndex :type Integer) (bFromSweep :type Boolean) (SweepResult :type Hit%20Result%20Structure%20%28by%20ref%29))
  (if (== OtherActor (Game|Player|GetPlayerPawn 0))
    (Utilities|FlowControl|Delay (Math|Random|RandomFloatinRange 0.0 2.0))
    (bind _returnvalue (Utilities|Time|SetTimerbyEvent (delegate Custom|StartSwingForward) 0.01 true))
    (Variables|Default|SetSwingTimer _returnvalue)))

(event OnComponentEndOverlap(StartSwingingVolume)
  (params (OverlappedComponent :type Primitive%20Component%20Object%20Reference) (OtherActor :type Actor%20Object%20Reference) (OtherComp :type Primitive%20Component%20Object%20Reference) (OtherBodyIndex :type Integer))
  (if (== OtherActor (Game|Player|GetPlayerPawn 0))
    (Utilities|Time|ClearandInvalidateTimerbyHandle (Variables|Default|GetSwingTimer))))

(event Custom|StartSwingForward
  (bind _lamp (Variables|Default|GetLamp))
  (Transformation|SetWorldRotation _lamp (Math|Rotator|MakeRotator (+ (Variables|Default|GetXValue) (.roll (Transformation|GetWorldRotation _lamp))) 0.0 0.0) false false)
  (Utilities|FlowControl|Sequence
    (:then_0
      (if (>= (+ (Variables|Default|GetXValue) (.roll (Transformation|GetWorldRotation _lamp))) (Math|Conversions|ToFloat(Integer) (Variables|Default|GetXValueLowPos)))
        (Variables|Default|SetXValue -0.1)))
    (:then_1
      (if (>= (+ (Variables|Default|GetXValue) (.roll (Transformation|GetWorldRotation _lamp))) (Math|Conversions|ToFloat(Integer) (Variables|Default|GetXValueHighPos)))
        (Variables|Default|SetXValue -0.2)))
    (:then_2
      (if (<= (+ (Variables|Default|GetXValue) (.roll (Transformation|GetWorldRotation _lamp))) (Math|Conversions|ToFloat(Integer) (Variables|Default|GetXValueLowNeg)))
        (Variables|Default|SetXValue 0.1)))
    (:then_3
      (if (<= (+ (Variables|Default|GetXValue) (.roll (Transformation|GetWorldRotation _lamp))) (Math|Conversions|ToFloat(Integer) (Variables|Default|GetXValueHighNeg)))
        (Variables|Default|SetXValue 0.2)))))

(event EventBeginPlay
  (Variables|Default|SetXValueLowPos (Math|Random|RandomIntegerinRange 20 25))
  (Variables|Default|SetXValueHighPos (Math|Random|RandomIntegerinRange 25 30))
  (Variables|Default|SetXValueLowNeg (Math|Random|RandomIntegerinRange -20 -25))
  (Variables|Default|SetXValueHighNeg (Math|Random|RandomIntegerinRange -25 -30)))

(fn ConstructionScript)