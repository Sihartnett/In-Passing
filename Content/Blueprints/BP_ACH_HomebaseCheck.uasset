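; BP_ACH_HomebaseCheck is a trigger actor that awards the OUTTA_HERE achievement.
; When the player pawn overlaps its Box, it reads flags from BP_GameMode and FirstPersonCharacter.
; It qualifies only if winged mode is unused, Ach4TouchedPlate is false and Ach4UsedKickball is true.
; It then caches achievements and, on success, writes progress for OUTTA_HERE to the player controller.
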(event OnComponentBeginOverlap(Box)
  (params (OverlappedComponent :type Primitive%20Component%20Object%20Reference) (OtherActor :type Actor%20Object%20Reference) (OtherComp :type Primitive%20Component%20Object%20Reference) (OtherBodyIndex :type Integer) (bFromSweep :type Boolean) (SweepResult :type Hit%20Result%20Structure%20%28by%20ref%29))
  (bind _returnvalue (Game|Player|GetPlayerPawn 0))
  (bind _returnvalue_2 (Game|GetPlayerController 0))
  (if (== OtherActor _returnvalue)
    (bind _asbp_game_mode (Utilities|Casting|CastToBP_GameMode (Game|GetGameMode)))
    (bind _asfirst_person_character (Utilities|Casting|CastToFirstPersonCharacter _returnvalue))
    (if (and (and (not (Variables|/Game/Blueprints/BP_GameMode.BP_GameMode_C|GetUsedWingedMode _asbp_game_mode)) (not (Variables|/Game/FirstPersonCPP/Blueprints/FirstPersonCharacter.FirstPersonCharacter_C|GetAch4_TouchedPlate _asfirst_person_character))) (Variables|/Game/FirstPersonCPP/Blueprints/FirstPersonCharacter.FirstPersonCharacter_C|GetAch4_UsedKickball _asfirst_person_character))
      (|CacheAchievements _returnvalue_2
        (:OnSuccess
          (|WriteAchievementProgress _returnvalue_2 "OUTTA_HERE" 1e+02))))))

(event EventBeginPlay)

(event Collision|EventActorBeginOverlap
  (params (OtherActor :type Actor%20Object%20Reference)))

(event EventTick
  (params (DeltaSeconds :type Float%20%28single-precision%29)))

(fn ConstructionScript)